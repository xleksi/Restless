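; BP_Item is a placeholder pickup actor that shows a widget component while something overlaps its Trigger and hides it when the overlap ends.
; The overlap events do not filter which actor entered or left.
; PickUpItem prints a debug message, calls DestroyItem and returns the Item variable.
; DestroyItem is an event that destroys the actor after a short delay, so the function itself returns immediately.
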(event `DestroyItem`
  (`KismetSystemLibrary.Delay` 0.1)
  (`self.K2_DestroyActor`))

(event `self.Trigger.OnComponentBeginOverlap`
  (params (OverlappedComponent :type "PrimitiveComponent Object Reference") (OtherActor :type "Actor Object Reference") (OtherComp :type "PrimitiveComponent Object Reference") (OtherBodyIndex :type Integer) (bFromSweep :type Boolean) (SweepResult :type "HitResult Structure (by ref)"))
  (`SceneComponent.SetVisibility` (`self.Widget`) true false))

(event `self.Trigger.OnComponentEndOverlap`
  (params (OverlappedComponent :type "PrimitiveComponent Object Reference") (OtherActor :type "Actor Object Reference") (OtherComp :type "PrimitiveComponent Object Reference") (OtherBodyIndex :type Integer))
  (`SceneComponent.SetVisibility` (`self.Widget`) false false))

(fn `PickUpItem`
  (returns (Item :type String))
  (`KismetSystemLibrary.PrintString` "Item Picked!")
  (`self.DestroyItem`)
  (return (`self.Item`)))

(fn `UserConstructionScript`)