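; BP_ItemParent is the parent Blueprint for interactable pickup items that go into the player's inventory.
; Interact destroys the actor and passes its class, icon and stack size to BP_ThirdPersonCharacter's AddItemToInventory.
; It first sends Door a key-pickup message if ItemClass equals the BP_HealthPotion actor found in the level.
; The overlap checks lead nowhere, PickUpItemMessage is unwired, and GetItemData returns only zeros.
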(event `self.ReceiveActorBeginOverlap`
  (params (OtherActor :type "Actor Object Reference"))
  (if (`KismetSystemLibrary.DoesImplementInterface` OtherActor "/Game/06UI/Inventory/BPI_Inventory.BPI_Inventory_C")
    (if (`KismetMathLibrary.ClassIsChildOf` (`GameplayStatics.GetObjectClass` OtherActor) "BP_ItemParent_C")
      _)))

(event `/Game/06UI/Inventory/BPI_Inventory.Interact`
  (bind _returnvalue (`GameplayStatics.GetActorOfClass` "/Game/00Placeholder/Interactables/BP_HealthPotion.BP_HealthPotion_C"))
  (if (== (`self.ItemClass`) _returnvalue)
    (message `/Game/06UI/Inventory/BPI_PickUpKey.PickUpKey` (`self.Door`)))
  (`self.K2_DestroyActor`)
  (bind _asbp_third_person_character (cast `/Game/ThirdPerson/Blueprints/BP_ThirdPersonCharacter` (`GameplayStatics.GetPlayerCharacter` 0)))
  (`/Game/ThirdPerson/Blueprints/BP_ThirdPersonCharacter.AddItemToInventory` _asbp_third_person_character (`self.ItemClass`) (`self.ItemIcon`) (`self.StackSize`)))

(fn `GetItemData`
  (returns (ItemClass :type "Actor Class Reference") (CurrentStackAmount :type Integer) (MaxStackAmount :type Integer))
  (return null 0 0))

(fn `UserConstructionScript`)