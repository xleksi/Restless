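; Placeholder interactable door that swings open when Interact fires.
; A timeline drives the Door component's yaw and calls UseItemMessage on the door's owner on every update.
; PickUpItem sets a HasKey flag and prints a debug string, but the key check in Interact has empty branches, so it does not gate opening.
; GetItemData is a stub returning zero stack amounts.
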(event `/Game/06UI/Inventory/BPI_Inventory.Interact`
  (if (`self.HasKey?`)
    (bind (_direction _open) (`Timeline|Open` :!label _label)
      (:`Update`
        (`SceneComponent.K2_SetRelativeRotation` (`self.Door`) (`KismetMathLibrary.MakeRotator` 0.0 0.0 _open) false false)
        (message `/Game/06UI/Inventory/BPI_Inventory.UseItem` (`self.GetOwner`))))
    (else
      (goto _label))))

(event `/Game/00Placeholder/Interactables/BPI_Door.PickUpItem`
  (set `self.HasKey?` true)
  (`KismetSystemLibrary.PrintString` "mee"))

(fn `GetItemData`
  (returns (ItemClass :type "Actor Class Reference") (CurrentStackAmount :type Integer) (MaxStackAmount :type Integer))
  (return null 0 0))

(fn `UserConstructionScript`)