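; BP_Door_2 is a placeholder interactable door that swings open when a player character holding a key enters its trigger box.
; Box overlap casts to BP_ThirdPersonCharacter, checks HasKey, then calls DoorOpen, where the Open timeline drives the Door's relative yaw.
; A key ID comparison through casting the door's owner to BP_Key_2 does not gate opening, and a debug "Hello" prints afterwards.
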(event `DoorOpen`
  (bind (_direction _open) (`Timeline|Open`)
    (:`Update`
      (`SceneComponent.K2_SetRelativeRotation` (`self.Door`) (`KismetMathLibrary.MakeRotator` 0.0 0.0 _open) false false))))

(event `self.Box.OnComponentBeginOverlap`
  (params (OverlappedComponent :type "PrimitiveComponent Object Reference") (OtherActor :type "Actor Object Reference") (OtherComp :type "PrimitiveComponent Object Reference") (OtherBodyIndex :type Integer) (bFromSweep :type Boolean) (SweepResult :type "HitResult Structure (by ref)"))
  (bind _asbp_third_person_character (cast `/Game/ThirdPerson/Blueprints/BP_ThirdPersonCharacter` OtherActor))
  (if (`/Game/ThirdPerson/Blueprints/BP_ThirdPersonCharacter.Has Key` _asbp_third_person_character)
    (bind _asbp_key_2 (cast `/Game/00Placeholder/Interactables/BP_Key_2` (`self.GetOwner`))
      (:`then`
        _)
      (:`CastFailed`
        _))
    (if (== (`/Game/00Placeholder/Interactables/BP_Key_2.NumberID` _asbp_key_2) (`self.NumberIDDoor`))
      _
      (else
        _))
    (`self.DoorOpen`)
    (`KismetSystemLibrary.PrintString` "Hello")))

(fn `UserConstructionScript`)