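; BP_Door is an interactable door that opens only after two separate keys have been picked up.
; Key pickup events store each item name, set HasKey once both are held, and show either a key-complete or second-key-needed widget.
; Interact plays the Open timeline to drive door yaw, sending UseItem messages for both keys to its owner on every update.
; A box overlap toggles the door's widget visibility.
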(event `/Game/00Placeholder/Interactables/DoorSystem/BPI_Interact.Interact`
  (bind _returnvalue (`self.GetOwner`))
  (if (`self.HasKey?`)
    (bind (_direction _open) (`Timeline|Open`)
      (:`Update`
        (`SceneComponent.K2_SetRelativeRotation` (`self.Door`) (`KismetMathLibrary.MakeRotator` 0.0 0.0 _open) false false)
        (message `/Game/06UI/Inventory/BPI_Inventory.UseItem` _returnvalue "/Game/00Placeholder/Interactables/DoorSystem/BP_Key1Child.BP_Key1Child_C" (`self.Key1Name`))
        (message `/Game/06UI/Inventory/BPI_Inventory.UseItem` _returnvalue "/Game/00Placeholder/Interactables/DoorSystem/BP_Key2Child.BP_Key2Child_C" (`self.Key2Name`))))))

(event `/Game/00Placeholder/Interactables/DoorSystem/BPI_Door.PickUpKey1`
  (params (ItemName :type Name))
  (set `self.Key1Name` ItemName)
  (set `self.hasKey1?` true)
  (if (and (`self.hasKey1?`) (`self.HasKey2?`)) :!label _label
    (set `self.HasKey?` true)
    (bind _returnvalue (`|CreateWidget` "/Game/06UI/Widgets/WBP_CompleteKey.WBP_CompleteKey_C"))
    (`UserWidget.AddToViewport` _returnvalue 0)
    (else
      (bind _returnvalue_2 (`|CreateWidget` "/Game/06UI/Widgets/WBP_NeedSecondeKey.WBP_NeedSecondeKey_C"))
      (`UserWidget.AddToViewport` _returnvalue_2 0))))

(event `/Game/00Placeholder/Interactables/DoorSystem/BPI_Door.PickUpKey2`
  (params (ItemName :type Name))
  (set `self.Key2Name` ItemName)
  (set `self.HasKey2?` true)
  (goto _label))

(event `self.Box.OnComponentBeginOverlap`
  (params (OverlappedComponent :type "PrimitiveComponent Object Reference") (OtherActor :type "Actor Object Reference") (OtherComp :type "PrimitiveComponent Object Reference") (OtherBodyIndex :type Integer) (bFromSweep :type Boolean) (SweepResult :type "HitResult Structure (by ref)"))
  (`SceneComponent.SetVisibility` (`self.Widget`) true false))

(event `self.Box.OnComponentEndOverlap`
  (params (OverlappedComponent :type "PrimitiveComponent Object Reference") (OtherActor :type "Actor Object Reference") (OtherComp :type "PrimitiveComponent Object Reference") (OtherBodyIndex :type Integer))
  (`SceneComponent.SetVisibility` (`self.Widget`) false false))

(fn `GetItemData`
  (returns (ItemClass :type "Actor Class Reference") (CurrentStackAmount :type Integer) (MaxStackAmount :type Integer))
  (return null 0 0))

(fn `UserConstructionScript`)