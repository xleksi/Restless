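; BP_InvisiblePotion is an interactable pickup that goes into the player's inventory.
; An overlap sphere shows its widget when something enters and hides it on exit.
; Interact casts the player character to BP_ThirdPersonCharacter, adds the item using its class, icon and stack size, then destroys the pickup.
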(event `self.OverlapSphere.OnComponentBeginOverlap`
  (params (OverlappedComponent :type "PrimitiveComponent Object Reference") (OtherActor :type "Actor Object Reference") (OtherComp :type "PrimitiveComponent Object Reference") (OtherBodyIndex :type Integer) (bFromSweep :type Boolean) (SweepResult :type "HitResult Structure (by ref)"))
  ;[1 1 1] Widget visibility
  (`SceneComponent.SetVisibility` (`self.Widget`) true false))

(event `self.OverlapSphere.OnComponentEndOverlap`
  (params (OverlappedComponent :type "PrimitiveComponent Object Reference") (OtherActor :type "Actor Object Reference") (OtherComp :type "PrimitiveComponent Object Reference") (OtherBodyIndex :type Integer))
  ;[1 1 1] Widget visibility
  (`SceneComponent.SetVisibility` (`self.Widget`) false false))

(event `/Game/00Placeholder/Interactables/DoorSystem/BPI_Interact.Interact`
  (bind _asbp_third_person_character (cast `/Game/ThirdPerson/Blueprints/BP_ThirdPersonCharacter` (`GameplayStatics.GetPlayerCharacter` 0)))
  (`/Game/ThirdPerson/Blueprints/BP_ThirdPersonCharacter.AddItemToInventory` _asbp_third_person_character (`self.ItemClass`) (`self.ItemIcon`) (`self.StackSize`))
  (`self.K2_DestroyActor`))

(fn `UserConstructionScript`
  (`parent.UserConstructionScript`))