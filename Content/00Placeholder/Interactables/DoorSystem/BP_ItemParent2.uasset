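; BP_ItemParent2 is a base pickup item that offers itself to inventory-capable actors that overlap it.
; On overlap it checks for BPI_Inventory, skips actors derived from its own class, then sends PickUpItemMessage with its item class, icon and stack size.
; The Interact event is empty, and the direct add-to-character-inventory and destroy chain is disconnected, so the item never destroys itself here.
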(event `self.ReceiveActorBeginOverlap`
  (params (OtherActor :type "Actor Object Reference"))
  (if (`KismetSystemLibrary.DoesImplementInterface` OtherActor "/Game/06UI/Inventory/BPI_Inventory.BPI_Inventory_C")
    (if (not (`KismetMathLibrary.ClassIsChildOf` (`GameplayStatics.GetObjectClass` OtherActor) "BP_ItemParent2_C"))
      (message `/Game/06UI/Inventory/BPI_Inventory.PickUpItem` OtherActor (`self.ItemClass`) (`self.ItemIcon`) (`self.StackSize`)))))

(event `/Game/00Placeholder/Interactables/DoorSystem/BPI_Interact.Interact`)

(fn `UserConstructionScript`)