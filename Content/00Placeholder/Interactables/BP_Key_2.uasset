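; BP_Key_2 is a placeholder key pickup that shows a widget while something overlaps its trigger.
; PickUpKey calls DestroyKey and returns Item.
; DestroyKey prints a message, waits briefly and destroys the actor, only then casting the key's owner to BP_ThirdPersonCharacter to set HasKey.
; The flag is set only if that owner cast succeeds, and nothing here assigns the owner.
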(event `DestroyKey`
  (`KismetSystemLibrary.PrintString` "Player has key")
  (`KismetSystemLibrary.Delay` 0.1)
  (`self.K2_DestroyActor`)
  (bind _asbp_third_person_character (cast `/Game/ThirdPerson/Blueprints/BP_ThirdPersonCharacter` (`self.GetOwner`)))
  (set `/Game/ThirdPerson/Blueprints/BP_ThirdPersonCharacter.Has Key` true _asbp_third_person_character))

(event `self.Trigger.OnComponentBeginOverlap`
  (params (OverlappedComponent :type "PrimitiveComponent Object Reference") (OtherActor :type "Actor Object Reference") (OtherComp :type "PrimitiveComponent Object Reference") (OtherBodyIndex :type Integer) (bFromSweep :type Boolean) (SweepResult :type "HitResult Structure (by ref)"))
  (`SceneComponent.SetVisibility` (`self.Widget`) true false))

(event `self.Trigger.OnComponentEndOverlap`
  (params (OverlappedComponent :type "PrimitiveComponent Object Reference") (OtherActor :type "Actor Object Reference") (OtherComp :type "PrimitiveComponent Object Reference") (OtherBodyIndex :type Integer))
  (`SceneComponent.SetVisibility` (`self.Widget`) false false))

(fn `PickUpKey`
  (returns (Item :type String))
  (`self.DestroyKey`)
  (return (`self.Item`)))

(fn `UserConstructionScript`)