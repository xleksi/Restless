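; BP_Drop is a placeholder jumpscare trigger that drops a sphere when the player enters its box.
; On BeginPlay it shows the sphere with physics off and hides the Button component.
; The first overlap by BP_ThirdPersonCharacter enables sphere physics through a DoOnce, then plays the Broken sound in 2D after a short fixed delay, with no impact detection.
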(event `self.ReceiveBeginPlay`
  (bind _sphere (`self.Sphere`))
  (`SceneComponent.SetVisibility` _sphere true false)
  (`PrimitiveComponent.SetSimulatePhysics` _sphere false)
  ;[1 0.8907 0.4691] developmentOnly
  (`SceneComponent.SetVisibility` (`self.button`) false false))

(event `self.Box.OnComponentBeginOverlap`
  (params (OverlappedComponent :type "PrimitiveComponent Object Reference") (OtherActor :type "Actor Object Reference") (OtherComp :type "PrimitiveComponent Object Reference") (OtherBodyIndex :type Integer) (bFromSweep :type Boolean) (SweepResult :type "HitResult Structure (by ref)"))
  (cast `/Game/ThirdPerson/Blueprints/BP_ThirdPersonCharacter` OtherActor)
  (`/Engine/EditorBlueprintResources/StandardMacros.DoOnce` false
    (:`Completed`
      (`PrimitiveComponent.SetSimulatePhysics` (`self.Sphere`) true)
      (`KismetSystemLibrary.Delay` 0.8)
      (`GameplayStatics.PlaySound2D` "/Game/04Sound/SoundPlaceholder/Broken.Broken" 1.0 1.0 0.0 null null))))

(fn `UserConstructionScript`)