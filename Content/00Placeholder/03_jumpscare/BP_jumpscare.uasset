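; BP_jumpscare is a one-time jumpscare actor that briefly flashes the BigDaddy component when the third-person player character enters its trigger.
; BigDaddy is hidden on BeginPlay.
; The first overlap passes a DoOnce, plays 2D white noise, disables the character's input and, after short delays, shows BigDaddy, then hides it and restores input.
; A second, unconnected copy of the sequence never runs.
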(event `self.ReceiveBeginPlay`
  (`SceneComponent.SetVisibility` (`self.Big_Daddy`) false false))

(event `self.jumpscare_trigger.OnComponentBeginOverlap`
  (params (OverlappedComponent :type "PrimitiveComponent Object Reference") (OtherActor :type "Actor Object Reference") (OtherComp :type "PrimitiveComponent Object Reference") (OtherBodyIndex :type Integer) (bFromSweep :type Boolean) (SweepResult :type "HitResult Structure (by ref)"))
  (bind _big_daddy (`self.Big_Daddy`))
  (bind _asbp_third_person_character (cast `/Game/ThirdPerson/Blueprints/BP_ThirdPersonCharacter` OtherActor))
  (`/Engine/EditorBlueprintResources/StandardMacros.DoOnce` false
    (:`Completed`
      (`GameplayStatics.PlaySound2D` "/Engine/EngineSounds/WhiteNoise.WhiteNoise" 1.0 1.0 0.0 null null)
      (`self.DisableInput` _asbp_third_person_character null)
      (`KismetSystemLibrary.Delay` 0.2)
      (`SceneComponent.SetVisibility` _big_daddy true false)
      (`KismetSystemLibrary.Delay` 0.5)
      (`self.EnableInput` _asbp_third_person_character null)
      (`SceneComponent.SetVisibility` _big_daddy false false))))

(fn `UserConstructionScript`)