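; BP_NoiseWooden is an overlap-triggered wooden noise source that makes the player character's presence audible when they touch it.
; When a BP_ThirdPersonCharacter overlaps it, it plays a wooden sound at its location and adds a new NoiseWood widget to the viewport.
; It also reports an AI perception noise event there with the character as instigator and prints a debug string.
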(event `self.ReceiveActorBeginOverlap`
  (params (OtherActor :type "Actor Object Reference"))
  (bind _returnvalue (`self.K2_GetActorLocation`))
  (cast `/Game/ThirdPerson/Blueprints/BP_ThirdPersonCharacter` OtherActor)
  (if true
    (`GameplayStatics.PlaySoundAtLocation` "/Game/04Sound/SoundPlaceholder/wooden_1_.wooden_1_" _returnvalue (struct) 1.0 1.0 0.0 null null null null)
    (bind _returnvalue_2 (`|CreateWidget` "/Game/06UI/Widgets/NoiseWood.NoiseWood_C"))
    (`UserWidget.AddToViewport` _returnvalue_2 0)
    (`AISense_Hearing.ReportNoiseEvent` _returnvalue 1.0 OtherActor)
    (`KismetSystemLibrary.PrintString` "Wooden Noise" true true (struct :`G` 1.0 :`B` 0.279283 :`A` 1.0))))

(fn `UserConstructionScript`)