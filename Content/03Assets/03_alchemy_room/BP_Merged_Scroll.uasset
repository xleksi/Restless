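; Interactable ancient scroll actor that opens a full-screen message widget when the player interacts with it.
; Look-at events toggle its prompt widget and pickup flag, and a map outline event toggles custom depth on the mesh for a matching ItemID.
; Interacting flags the character as viewing a widget, hides the cursor and, only if no valid scroll widget exists, creates one and switches input to UI only.
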(event `/Game/03Assets/BI_HighLightCommuncation.LookAtItem`
  (params (`?LookAt` :type Boolean))
  (`SceneComponent.SetVisibility` (`self.Widget`) `?LookAt` false)
  (set `self.?AbleToPickUp` `?LookAt`))

(event `/Game/03Assets/BI_HighLightCommuncation.OutlineOnMap`
  (params (`?Outline` :type Boolean) (NumberID :type "Float (double-precision)"))
  (if (== NumberID (`self.ItemID`))
    (`PrimitiveComponent.SetRenderCustomDepth` (`self.old__ancient_scroll`) `?Outline`)))

(event `/Game/03Assets/BI_HighLightCommuncation.InteractItem`
  (bind _asbp_third_person_character (cast `/Game/ThirdPerson/Blueprints/BP_ThirdPersonCharacter` (`GameplayStatics.GetPlayerCharacter` 0)))
  (set `/Game/ThirdPerson/Blueprints/BP_ThirdPersonCharacter.?LookingAtWidget` true _asbp_third_person_character)
  (set `PlayerController.bShowMouseCursor` false (`GameplayStatics.GetPlayerController` 0))
  (`self.scroll message`
    (:`then`)
    (:`else`
      ;[1 0.8805 0] Comment
      (bind _returnvalue (`|CreateWidget` "/Game/00GUIDE_CLUES/WBP_5_scroll.WBP_5_scroll_C"))
      (bind _output_get (set `self.scroll message` _returnvalue))
      (`UserWidget.AddToViewport` _output_get 0)
      (`WidgetBlueprintLibrary.SetInputMode_UIOnlyEx` (`GameplayStatics.GetPlayerController` 0) (`self.scroll message`)))))

(fn `IsAbleToBePickedUp`
  (returns (`?AbleToPickUp` :type Boolean))
  (return (`self.?AbleToPickUp`)))

(fn `UserConstructionScript`)