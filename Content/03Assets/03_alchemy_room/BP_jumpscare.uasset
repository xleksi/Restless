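; One-shot jumpscare actor for the alchemy room that flashes four hidden ghosts at the player.
; When the third-person character overlaps the trigger, it plays white noise, disables input, shows the ghosts and quickly blends the view to this actor.
; After a short delay it restores input, hides the ghosts and blends the view back to the character.
; A similar, older-looking node chain is left unconnected.
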(event `self.ReceiveBeginPlay`
  (`SceneComponent.SetVisibility` (`self.ghost1`) false false)
  (`SceneComponent.SetVisibility` (`self.Ghost0`) false false)
  (`SceneComponent.SetVisibility` (`self.ghost3`) false false)
  (`SceneComponent.SetVisibility` (`self.ghost2`) false false))

(event `self.jumpscare_trigger.OnComponentBeginOverlap`
  (params (OverlappedComponent :type "PrimitiveComponent Object Reference") (OtherActor :type "Actor Object Reference") (OtherComp :type "PrimitiveComponent Object Reference") (OtherBodyIndex :type Integer) (bFromSweep :type Boolean) (SweepResult :type "HitResult Structure (by ref)"))
  (bind _ghost1 (`self.ghost1`))
  (bind _asbp_third_person_character (cast `/Game/ThirdPerson/Blueprints/BP_ThirdPersonCharacter` OtherActor))
  (`/Engine/EditorBlueprintResources/StandardMacros.DoOnce` false
    (:`Completed`
      (`GameplayStatics.PlaySound2D` "/Engine/EngineSounds/WhiteNoise.WhiteNoise" 1.0 1.0 0.0 null null)
      (`self.DisableInput` _asbp_third_person_character null)
      (`SceneComponent.SetVisibility` _ghost1 true false)
      (`SceneComponent.SetVisibility` (`self.ghost2`) true false)
      (`SceneComponent.SetVisibility` (`self.ghost3`) true false)
      (`SceneComponent.SetVisibility` (`self.Ghost0`) true false)
      ;[1 0.9822 0.2473] blend time(camera rotation time)
      (`PlayerController.SetViewTargetWithBlend` (`GameplayStatics.GetPlayerController` 0) self 0.1 "VTBlend_Linear" 0.0 false)
      (`KismetSystemLibrary.Delay` 0.4)
      (`self.EnableInput` _asbp_third_person_character null)
      (`SceneComponent.SetVisibility` _ghost1 false false)
      (`SceneComponent.SetVisibility` (`self.ghost2`) false false)
      (`SceneComponent.SetVisibility` (`self.ghost3`) false false)
      (`SceneComponent.SetVisibility` (`self.Ghost0`) false false)
      (`PlayerController.SetViewTargetWithBlend` (`GameplayStatics.GetPlayerController` 0) _asbp_third_person_character 0.1 "VTBlend_Linear" 0.0 false))))

(fn `UserConstructionScript`)