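; Door blocked by planks that the player chops away with an equipped weapon, after which it swings open.
; The NearDoor trigger shows one of two prompt widgets depending on the weapon, enabling attack on the character when armed.
; DestroyPlank runs a timed sequence of chop sound, physics-simulated plank break, unlock sound and timeline-driven rotation.
; A CloseDoor trigger clears weapon messages through BI_Weapons and reverses a second timeline to shut the door once.
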(event `self.ReceiveBeginPlay`
  (set `self.WidgetArray` (`|MakeArray` (`self.DestroyPlanks`) (`self.NearDoorWidget`))))

(event `DestroyPlank`
  ;[1 1 1] Opening Door
  ;;[1 0.9289 0] wait axe animation finished
  (`KismetSystemLibrary.Delay` 1.5)
  ;;[1 0.8392 0.01883] chaotic simulation
  (`GameplayStatics.PlaySound2D` "/Game/04Sound/chop_plank.chop_plank" 1.0 1.0 0.0 null null)
  (`PrimitiveComponent.SetSimulatePhysics` (`self.destroy_planks_chaotic`) true)
  (`KismetSystemLibrary.Delay` 2.0)
  ;;[1 0.8392 0.01883] sfx_unlock the door
  (`GameplayStatics.PlaySound2D` "/Game/04Sound/SFX_interaction/sfx_louder_unlock_the_door_ncc0.sfx_louder_unlock_the_door_ncc0" 1.0 1.0 0.0 null null)
  (bind (_direction _open) (`Timeline|Open`)
    (:`Update`
      (`SceneComponent.K2_SetRelativeRotation` (`self.SketchFab_FBX_All_Modules_door`) (`KismetMathLibrary.MakeRotator` 0.0 0.0 _open) false false))
    (:`Finished`
      (bind _asbp_third_person_character (cast `/Game/ThirdPerson/Blueprints/BP_ThirdPersonCharacter` (`GameplayStatics.GetPlayerCharacter` 0)))
      (set `/Game/ThirdPerson/Blueprints/BP_ThirdPersonCharacter.?NearPlanks` false _asbp_third_person_character)
      (set `/Game/ThirdPerson/Blueprints/BP_ThirdPersonCharacter.?CanAttack` false _asbp_third_person_character)
      (for _array_element (`self.WidgetArray`)
        (`SceneComponent.SetVisibility` _array_element false false)
        (set `self.?DoorOpen` true)))))

(event `self.NearDoor.OnComponentBeginOverlap`
  (params (OverlappedComponent :type "PrimitiveComponent Object Reference") (OtherActor :type "Actor Object Reference") (OtherComp :type "PrimitiveComponent Object Reference") (OtherBodyIndex :type Integer) (bFromSweep :type Boolean) (SweepResult :type "HitResult Structure (by ref)"))
  (if (== OtherActor (`GameplayStatics.GetPlayerCharacter` 0))
    (if (not (`self.?DoorOpen`))
      (bind _asbp_third_person_character (cast `/Game/ThirdPerson/Blueprints/BP_ThirdPersonCharacter` (`GameplayStatics.GetPlayerCharacter` 0)))
      (if (`/Game/ThirdPerson/Blueprints/BP_ThirdPersonCharacter.?WeaponEquiped` _asbp_third_person_character)
        (`SceneComponent.SetVisibility` (`self.DestroyPlanks`) true false)
        (set `/Game/ThirdPerson/Blueprints/BP_ThirdPersonCharacter.?NearPlanks` true _asbp_third_person_character)
        (set `/Game/ThirdPerson/Blueprints/BP_ThirdPersonCharacter.?CanAttack` true _asbp_third_person_character)
        (else
          (`SceneComponent.SetVisibility` (`self.NearDoorWidget`) true false))))))

(event `self.NearDoor.OnComponentEndOverlap`
  (params (OverlappedComponent :type "PrimitiveComponent Object Reference") (OtherActor :type "Actor Object Reference") (OtherComp :type "PrimitiveComponent Object Reference") (OtherBodyIndex :type Integer))
  (if (== (`GameplayStatics.GetPlayerCharacter` 0) OtherActor)
    (if (not (`self.?DoorOpen`))
      (for _array_element (`self.WidgetArray`)
        (`SceneComponent.SetVisibility` _array_element false false)))))

(event `self.Close Door.OnComponentBeginOverlap`
  (params (OverlappedComponent :type "PrimitiveComponent Object Reference") (OtherActor :type "Actor Object Reference") (OtherComp :type "PrimitiveComponent Object Reference") (OtherBodyIndex :type Integer) (bFromSweep :type Boolean) (SweepResult :type "HitResult Structure (by ref)"))
  ;[1 1 1] close door
  (if (`self.?DoorOpen`)
    (if (`self.?ClosedDoor`)
      _
      (elif (== OtherActor (`GameplayStatics.GetPlayerCharacter` 0))
        (bind _foundwidgets (`WidgetBlueprintLibrary.GetAllWidgetsWithInterface` "/Game/06UI/Inventory/Interfaces/BI_Weapons.BI_Weapons_C"))
        (for _array_element _foundwidgets
          (message `/Game/06UI/Inventory/Interfaces/BI_Weapons.RemoveWeapon` _array_element false))
        (bind (_direction _open) (`Timeline|Timeline` :!via `Reverse`)
          (:`Update`
            (`SceneComponent.K2_SetRelativeRotation` (`self.SketchFab_FBX_All_Modules_door`) (`KismetMathLibrary.MakeRotator` 0.0 0.0 _open) false false))
          (:`Finished`
            (set `self.?ClosedDoor` true)))))))

(fn `UserConstructionScript`)