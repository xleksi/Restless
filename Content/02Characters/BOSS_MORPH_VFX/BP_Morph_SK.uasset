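; Boss morph VFX actor that visually transitions the boss from its walking mesh to its post-morph body, hair, cloth and tentacle meshes.
; BeginPlay creates dynamic materials, hides the tentacle, hair and body, then reveals them after a fixed delay.
; A timeline drives the "Animation" scalar on the walking mesh's materials, and its update plays a second timeline driving the morphed parts.
; Niagara skeletal mesh overrides are present but unconnected.
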(event `self.ReceiveBeginPlay`
  (bind _bosswalk_before (`self.bosswalk_before`))
  (bind _returnvalue (`PrimitiveComponent.CreateDynamicMaterialInstance` _bosswalk_before 0 null "None"))
  (set `self.dynamic_material0` _returnvalue)
  (bind _returnvalue_2 (`PrimitiveComponent.CreateDynamicMaterialInstance` _bosswalk_before 1 null "None"))
  (set `self.dynamic_material1` _returnvalue_2)
  (bind _returnvalue_3 (`PrimitiveComponent.CreateDynamicMaterialInstance` _bosswalk_before 2 null "None"))
  (set `self.dynamic_material2` _returnvalue_3)
  (bind _returnvalue_4 (`PrimitiveComponent.CreateDynamicMaterialInstance` _bosswalk_before 3 null "None"))
  (set `self.dynamic_material3` _returnvalue_4)
  (bind _returnvalue_5 (`PrimitiveComponent.CreateDynamicMaterialInstance` _bosswalk_before 4 null "None"))
  (set `self.dynamic_material4` _returnvalue_5)
  (bind _returnvalue_6 (`PrimitiveComponent.CreateDynamicMaterialInstance` _bosswalk_before 5 null "None"))
  (set `self.dynamic_material5` _returnvalue_6)
  ;[0.9976 1 0] tentacle dynamic material
  (bind _returnvalue_7 (`PrimitiveComponent.CreateDynamicMaterialInstance` (`self.tentacle`) 0 null "None"))
  (set `self.Dy_8_tentacle` _returnvalue_7)
  (bind _returnvalue_8 (`PrimitiveComponent.CreateDynamicMaterialInstance` (`self.cloth_morph_after`) 0 null "None"))
  (set `self.dy9_cloth_fightmode` _returnvalue_8)
  (bind _returnvalue_9 (`PrimitiveComponent.CreateDynamicMaterialInstance` (`self.hair_morph_after`) 0 null "None"))
  (set `self.dyhair` _returnvalue_9)
  (bind _returnvalue_10 (`PrimitiveComponent.CreateDynamicMaterialInstance` (`self.Boss_body_morph_after`) 0 null "None"))
  (set `self.dy_body` _returnvalue_10)
  ;[1 0.9744 0] visibility
  (`SceneComponent.SetVisibility` (`self.tentacle`) false false)
  (`SceneComponent.SetVisibility` (`self.hair_morph_after`) false false)
  (`SceneComponent.SetVisibility` (`self.Boss_body_morph_after`) false false)
  (`SceneComponent.SetVisibility` (`self.hair_morph_after`) false false)
  (`KismetSystemLibrary.Delay` 4.8)
  (`SceneComponent.SetVisibility` (`self.tentacle`) true false)
  (`SceneComponent.SetVisibility` (`self.Boss_body_morph_after`) true false)
  (`SceneComponent.SetVisibility` (`self.hair_morph_after`) true false)
  (bind (_direction _newtrack_0) (`Timeline|Timeline`)
    (:`Update`
      (`MaterialInstanceDynamic.SetScalarParameterValue` (`self.dynamic_material0`) "Animation" _newtrack_0)
      (`MaterialInstanceDynamic.SetScalarParameterValue` (`self.dynamic_material1`) "Animation" _newtrack_0)
      (`MaterialInstanceDynamic.SetScalarParameterValue` (`self.dynamic_material2`) "Animation" _newtrack_0)
      (`MaterialInstanceDynamic.SetScalarParameterValue` (`self.dynamic_material3`) "Animation" _newtrack_0)
      (`MaterialInstanceDynamic.SetScalarParameterValue` (`self.dynamic_material4`) "Animation" _newtrack_0)
      (`MaterialInstanceDynamic.SetScalarParameterValue` (`self.dynamic_material5`) "Animation" _newtrack_0)
      (bind (_direction_2 _newtrack_0_2) (`Timeline|Timeline_0`)
        (:`Update`
          (`MaterialInstanceDynamic.SetScalarParameterValue` (`self.Dy_8_tentacle`) "Animation" _newtrack_0_2)
          (`MaterialInstanceDynamic.SetScalarParameterValue` (`self.dyhair`) "Animation" _newtrack_0_2)
          (`MaterialInstanceDynamic.SetScalarParameterValue` (`self.dy9_cloth_fightmode`) "Animation" _newtrack_0_2)
          (`MaterialInstanceDynamic.SetScalarParameterValue` (`self.dy_body`) "Animation" _newtrack_0_2))))))

(fn `UserConstructionScript`)