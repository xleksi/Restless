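; Boss transformation actor that morphs the walking boss mesh into its fight-mode body, tentacle and head through animated materials and Niagara.
; On BeginPlay it creates dynamic materials, hides the fight-mode parts, then after a delay shows all but the head and binds Niagara to the walk mesh.
; Two timelines drive the "Animation" parameter, the second started from the first's update, and the head appears when the first finishes.
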(event `self.ReceiveBeginPlay`
  (bind _niagara (`self.Niagara`))
  (bind _bosswalk (`self.bosswalk`))
  (bind _sm_merged_fightmode (`self.SM_MERGED_fightmode`))
  (bind _bosswalk_2 (`self.bosswalk`))
  (bind _returnvalue (`PrimitiveComponent.CreateDynamicMaterialInstance` _bosswalk 0 null "None"))
  (set `self.dynamic_material0` _returnvalue)
  (bind _returnvalue_2 (`PrimitiveComponent.CreateDynamicMaterialInstance` _bosswalk 1 null "None"))
  (set `self.dynamic_material1` _returnvalue_2)
  (bind _returnvalue_3 (`PrimitiveComponent.CreateDynamicMaterialInstance` _bosswalk 2 null "None"))
  (set `self.dynamic_material2` _returnvalue_3)
  (bind _returnvalue_4 (`PrimitiveComponent.CreateDynamicMaterialInstance` _bosswalk 3 null "None"))
  (set `self.dynamic_material3` _returnvalue_4)
  (bind _returnvalue_5 (`PrimitiveComponent.CreateDynamicMaterialInstance` _bosswalk 4 null "None"))
  (set `self.dynamic_material4` _returnvalue_5)
  (bind _returnvalue_6 (`PrimitiveComponent.CreateDynamicMaterialInstance` _bosswalk 5 null "None"))
  (set `self.dynamic_material5` _returnvalue_6)
  (bind _returnvalue_7 (`PrimitiveComponent.CreateDynamicMaterialInstance` _bosswalk 6 null "None"))
  (set `self.dynamic_material6` _returnvalue_7)
  (bind _returnvalue_8 (`PrimitiveComponent.CreateDynamicMaterialInstance` _bosswalk 7 null "None"))
  (set `self.dynamic_material7` _returnvalue_8)
  ;[0.9976 1 0] tentacle dynamic material
  (bind _returnvalue_9 (`PrimitiveComponent.CreateDynamicMaterialInstance` (`self.tentacle`) 0 null "None"))
  (set `self.Dynamic_8` _returnvalue_9)
  (bind _returnvalue_10 (`PrimitiveComponent.CreateDynamicMaterialInstance` _sm_merged_fightmode 0 null "None"))
  (set `self.dy9` _returnvalue_10)
  (bind _returnvalue_11 (`PrimitiveComponent.CreateDynamicMaterialInstance` _sm_merged_fightmode 1 null "None"))
  (set `self.dy10` _returnvalue_11)
  (bind _returnvalue_12 (`PrimitiveComponent.CreateDynamicMaterialInstance` _sm_merged_fightmode 2 null "None"))
  (set `self.dy11` _returnvalue_12)
  (bind _returnvalue_13 (`PrimitiveComponent.CreateDynamicMaterialInstance` (`self.boss_body_withoutleg`) 0 null "None"))
  (set `self.dy12` _returnvalue_13)
  (`SceneComponent.SetVisibility` (`self.MH_Bosshead2`) false false)
  (`SceneComponent.SetVisibility` (`self.SM_MERGED_fightmode`) false false)
  (`SceneComponent.SetVisibility` (`self.boss_body_withoutleg`) false false)
  (`SceneComponent.SetVisibility` (`self.tentacle`) false false)
  (`KismetSystemLibrary.Delay` 2.2)
  (`SceneComponent.SetVisibility` (`self.tentacle`) true false)
  (`SceneComponent.SetVisibility` (`self.SM_MERGED_fightmode`) true false)
  (`SceneComponent.SetVisibility` (`self.boss_body_withoutleg`) true false)
  (`NiagaraFunctionLibrary.OverrideSystemUserVariableSkeletalMeshComponent` _niagara "Skeletal Mesh0" _bosswalk_2)
  (`NiagaraFunctionLibrary.OverrideSystemUserVariableSkeletalMeshComponent` _niagara "Skeletal Mesh1" _bosswalk_2)
  (bind (_direction _newtrack_0) (`Timeline|Timeline`)
    (:`Update`
      (`MaterialInstanceDynamic.SetScalarParameterValue` (`self.dynamic_material0`) "Animation" _newtrack_0)
      (`MaterialInstanceDynamic.SetScalarParameterValue` (`self.dynamic_material1`) "Animation" _newtrack_0)
      (`MaterialInstanceDynamic.SetScalarParameterValue` (`self.dynamic_material2`) "Animation" _newtrack_0)
      (`MaterialInstanceDynamic.SetScalarParameterValue` (`self.dynamic_material3`) "Animation" _newtrack_0)
      (`MaterialInstanceDynamic.SetScalarParameterValue` (`self.dynamic_material4`) "Animation" _newtrack_0)
      (`MaterialInstanceDynamic.SetScalarParameterValue` (`self.dynamic_material5`) "Animation" _newtrack_0)
      (`MaterialInstanceDynamic.SetScalarParameterValue` (`self.dynamic_material6`) "Animation" _newtrack_0)
      (`MaterialInstanceDynamic.SetScalarParameterValue` (`self.dynamic_material7`) "Animation" _newtrack_0)
      (bind (_direction_2 _newtrack_0_2) (`Timeline|Timeline_0`)
        (:`Update`
          (`MaterialInstanceDynamic.SetScalarParameterValue` (`self.Dynamic_8`) "Animation" _newtrack_0_2)
          (`MaterialInstanceDynamic.SetScalarParameterValue` (`self.dy9`) "Animation" _newtrack_0_2)
          (`MaterialInstanceDynamic.SetScalarParameterValue` (`self.dy10`) "Animation" _newtrack_0_2)
          (`MaterialInstanceDynamic.SetScalarParameterValue` (`self.dy11`) "Animation" _newtrack_0_2)
          (`MaterialInstanceDynamic.SetScalarParameterValue` (`self.dy12`) "Animation" _newtrack_0_2))))
    (:`Finished`
      (`SceneComponent.SetVisibility` (`self.MH_Bosshead2`) true false))))

(fn `UserConstructionScript`)