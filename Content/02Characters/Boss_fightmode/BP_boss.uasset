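; Boss enemy for fight mode that yaws to face the player every tick and attacks in a self-repeating loop after a short start delay.
; Player distance, bucketed per 1000 units, picks chakra, sword slam, triple javelin or single javelin, each a spawned attack actor with its own cooldown.
; Each hit removes fixed health; death animates a material parameter before destroying the actor, clears the health bar and shows the win screen.
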(event `self.ReceiveBeginPlay`
  (`KismetSystemLibrary.Delay` 3.0)
  (`self.BossAttack`))

(event `self.ReceiveTick`
  (params (DeltaSeconds :type "Float (single-precision)"))
  (bind (_returnvalue_roll _returnvalue_pitch _returnvalue_yaw) (`KismetMathLibrary.BreakRotator` (`KismetMathLibrary.FindLookAtRotation` (`self.K2_GetActorLocation`) (`self.K2_GetActorLocation` (`GameplayStatics.GetPlayerCharacter` 0)))))
  ;[1 1 1] boss face to player
  (`self.K2_SetActorRotation` (`KismetMathLibrary.MakeRotator` 0.0 0.0 _returnvalue_yaw)))

(event `BossAttack`
  (bind (_returnvalue_x _returnvalue_y _returnvalue_z) (`KismetMathLibrary.BreakVector` (`self.K2_GetActorLocation`)))
  ;[1 0.9848 0.217] play energize animation if have one
  (`self.PlayAnimMontage` null)
  ;[1 1 1] 4 types of attack
  (switch `int` (`KismetMathLibrary.FTrunc` (/ (`KismetMathLibrary.Vector_Distance` (`self.K2_GetActorLocation`) (`self.K2_GetActorLocation` (`GameplayStatics.GetPlayerCharacter` 0))) 1000.0))
    (:`Default`
      (bind _returnvalue (`|SpawnActorFromClass` "/Game/02Characters/BossBP_sword/Attack_Javelin.Attack_Javelin_C" (`KismetMathLibrary.MakeTransform` (+ (`self.K2_GetActorLocation`) (0.0 0.0 820.0))) "Undefined" "OverrideRootScale" null null :!label _label))
      (set `/Game/02Characters/BossBP_sword/Attack_Javelin.AttackOffset` (0.0 0.0 -50.0) _returnvalue)
      (`KismetSystemLibrary.Delay` 1.5)
      (`self.BossAttack` :!label _label_2))
    (:`0`
      (`|SpawnActorFromClass` "/Game/02Characters/BossBP_sword/Attack_chakra.Attack_chakra_C" (`KismetMathLibrary.MakeTransform` (`KismetMathLibrary.MakeVector` _returnvalue_x _returnvalue_y (- _returnvalue_z 200.0))) "AlwaysSpawn" "MultiplyWithRoot" null null :!label _label_3)
      (`KismetSystemLibrary.Delay` 5.0)
      (goto _label_2))
    (:`1`
      (goto _label_3))
    (:`2`
      (bind _returnvalue_2 (`|SpawnActorFromClass` "/Game/02Characters/BossBP_sword/AttackBase.AttackBase_C" (`KismetMathLibrary.MakeTransform` (- (`self.K2_GetActorLocation`) (0.0 0.0 400.0))) "AlwaysSpawn" "MultiplyWithRoot" null null))
      (`/Game/02Characters/BossBP_sword/AttackBase.charge` _returnvalue_2 0.0)
      (`KismetSystemLibrary.Delay` 3.0)
      (goto _label_2))
    (:`3`
      (`KismetArrayLibrary.Array_Clear` (`self.Javelins`) :!label _label_4)
      (for _index (range -1 2)
        (bind _returnvalue_3 (* _index 500.0))
        (bind _returnvalue_4 (`|SpawnActorFromClass` "/Game/02Characters/BossBP_sword/Attack_Javelin.Attack_Javelin_C" (`KismetMathLibrary.MakeTransform` (`self.Get Javelin Location` _returnvalue_3)) "Undefined" "OverrideRootScale" null null))
        (`KismetArrayLibrary.Array_Add` (`self.Javelins`) _returnvalue_4)
        (set `/Game/02Characters/BossBP_sword/Attack_Javelin.AttackOffset` (`KismetMathLibrary.MakeVector` _returnvalue_3 _returnvalue_3 -100.0) _returnvalue_4)
        (`/Game/02Characters/BossBP_sword/AttackBase.charge` _returnvalue_4 (* (+ _index 1) 0.3))
        (`KismetSystemLibrary.Delay` 1.8)
        (goto _label_2)))
    (:`4`
      (goto _label_4))
    (:`5`
      (goto _label_4))
    (:`6`
      (goto _label_4))
    (:`7`
      (goto _label))))

(event `death vfx`
  (bind _returnvalue (`PrimitiveComponent.CreateDynamicMaterialInstance` (`self.Boss_morphing_clothes`) 0 null "None"))
  (bind _returnvalue_2 (`PrimitiveComponent.CreateDynamicMaterialInstance` (`self.Boss_morphing_hair`) 0 null "None"))
  (bind _returnvalue_3 (`PrimitiveComponent.CreateDynamicMaterialInstance` (`self.tentacles`) 0 null "None"))
  (bind _returnvalue_4 (`PrimitiveComponent.CreateDynamicMaterialInstance` (`self.Boss_morphing_newhead`) 0 null "None"))
  (bind (_direction _newtrack_0) (`Timeline|Timeline`)
    (:`Update`
      (`MaterialInstanceDynamic.SetScalarParameterValue` _returnvalue "Animation" _newtrack_0)
      (`MaterialInstanceDynamic.SetScalarParameterValue` _returnvalue_2 "Animation" _newtrack_0)
      (`MaterialInstanceDynamic.SetScalarParameterValue` _returnvalue_3 "Animation" _newtrack_0)
      (`MaterialInstanceDynamic.SetScalarParameterValue` _returnvalue_4 "Animation" _newtrack_0))
    (:`Finished`
      (`self.K2_DestroyActor`))))

(event `show win end screen`
  (bind _returnvalue (`GameplayStatics.GetPlayerController` 0))
  (`KismetSystemLibrary.Delay` 2.0)
  (bind _returnvalue_2 (`|CreateWidget` "/Game/06UI/EndScreen/WBP_Endscreen.WBP_Endscreen_C"))
  (`UserWidget.AddToViewport` _returnvalue_2 0)
  (set `PlayerController.bShowMouseCursor` true _returnvalue)
  (`WidgetBlueprintLibrary.SetInputMode_UIOnlyEx` _returnvalue _returnvalue_2))

(fn `DamageTakenBoss`
  (set `self.BossHealth` (- (`self.BossHealth`) 25.0))
  (if (<= (`self.BossHealth`) 0.0)
    ;[1 0.9727 0] Comment
    (`self.death vfx`)
    (bind _foundwidgets (`WidgetBlueprintLibrary.GetAllWidgetsOfClass` "/Game/06UI/Widgets/WBP_BossHealthbar.WBP_BossHealthbar_C"))
    (for _array_element _foundwidgets
      (`Widget.RemoveFromParent` _array_element))
    (`self.show win end screen`)
    (return)))

(fn `UserConstructionScript`)