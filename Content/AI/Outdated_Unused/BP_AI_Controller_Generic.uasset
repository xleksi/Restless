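; Generic AI controller that runs the BT_AI behavior tree and feeds sight and hearing perception into its blackboard for chasing or investigating.
; Seeing a non-hiding BP_ThirdPersonCharacter stores it as target with its location and disables hearing.
; Any other stimulus from that character, including noise, clears the target and re-enables hearing.
; Hearing stimuli from any actor write a separate investigation location.
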(event `self.ReceiveBeginPlay`
  (`self.RunBehaviorTree` "/Game/AI/Outdated_Unused/BT_AI.BT_AI"))

(event `self.AIPerception.OnTargetPerceptionUpdated`
  (params (Actor :type "Actor Object Reference") (Stimulus :type "AIStimulus Structure"))
  ;[1 1 1] Detect and Chase/Investigate Target
  (`self.SightDetection` Actor Stimulus)
  (`self.HearingDetection` Actor Stimulus))

(fn `HearingDetection`
  (params (Actor :type "Actor Object Reference") (Stimulus :type "AIStimulus Structure"))
  (bind _returnvalue (`AIPerceptionSystem.GetSenseClassForStimulus` Stimulus))
  (if (== _returnvalue "/Script/AIModule.AISense_Hearing")
    (`BlackboardComponent.SetValueAsVector` (`AIBlueprintHelperLibrary.GetBlackboard` null) "InvestigationLocation" (`.StimulusLocation` (break `AIStimulus` Stimulus)))))

(fn `SightDetection`
  (params (Actor :type "Actor Object Reference") (Stimulus :type "AIStimulus Structure"))
  (bind (_age _expirationage _strength _stimuluslocation _receiverlocation _tag _bsuccessfullysensed) (break `AIStimulus` Stimulus))
  (bind _returnvalue (`AIBlueprintHelperLibrary.GetBlackboard` null))
  (bind _returnvalue_2 (`AIPerceptionSystem.GetSenseClassForStimulus` Stimulus))
  (bind _asbp_third_person_character (cast `/Game/ThirdPerson/Blueprints/BP_ThirdPersonCharacter` Actor))
  (if (and (not (`/Game/ThirdPerson/Blueprints/BP_ThirdPersonCharacter.IsHiding` _asbp_third_person_character)) (== _returnvalue_2 "/Script/AIModule.AISense_Sight") _bsuccessfullysensed)
    (`BlackboardComponent.SetValueAsVector` _returnvalue "VisualInvestigationLocation" _stimuluslocation)
    (`BlackboardComponent.SetValueAsObject` _returnvalue (`self.TargetActorName`) Actor)
    (`AIPerceptionComponent.SetSenseEnabled` (`self.AIPerception`) "/Script/AIModule.AISense_Hearing" false)
    (else
      (`BlackboardComponent.SetValueAsObject` (`AIBlueprintHelperLibrary.GetBlackboard` null) (`self.TargetActorName`) null)
      (`AIPerceptionComponent.SetSenseEnabled` (`self.AIPerception`) "/Script/AIModule.AISense_Hearing" true))))

(fn `UserConstructionScript`)