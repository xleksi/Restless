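; Sliding picture puzzle minigame actor, with tile movement not yet implemented.
; The construction script builds a grid of box spaces and mesh tiles with one empty corner, then optionally shuffles tile positions.
; Dynamic materials give each tile its texture offset to show a slice of one image.
; At play, the cursor shows and clicks store the tile and play a shutter sound; the sphere-overlap neighbor search is unwired.
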(event Custom|Meshclicked
  (params (TouchedComponent :type Primitive%20Component%20Object%20Reference) (ButtonPressed :type Key%20Structure :default "None"))
  (bind _output_get (Variables|Default|SetClicked%20Mesh TouchedComponent))
  (EventDispatchers|BindEventtoOnClicked _output_get (delegate Custom|Meshclicked))
  (Audio|PlaySound2D "/Engine/VREditor/Sounds/UI/Camera_Shutter.Camera_Shutter" 1.0 1.0 0.0 0 0)
  (Development|PrintString (Utilities|String|ToString(Integer) (stale _array_index))))

(event EventBeginPlay
  (Variables|/Script/Engine.PlayerController|SetbShowMouseCursor (Game|GetPlayerController 0) true)
  (for _array_element (Variables|Default|GetMesheslist)
    (EventDispatchers|BindEventtoOnClicked _array_element (delegate Custom|Meshclicked))))

(fn ConstructionScript
  (CallFunction|SpawnPuzzle)
  (CallFunction|ShufflePuzzle))

(fn SpawnPuzzle
  (bind _gridsize (Variables|Default|Getgridsize))
  (bind _mesh_size (Variables|Default|GetMesh_Size))
  (bind _gridsize_2 (Variables|Default|Getgridsize))
  (bind _spaceslist (Variables|Default|GetSpaceslist))
  (bind _mesheslist (Variables|Default|GetMesheslist))
  (bind _mesh_size_2 (Variables|Default|GetMesh_Size))
  (bind _gridsize_3 (Variables|Default|Getgridsize))
  (bind _returnvalue (Math|Conversions|ToFloat(Integer) _gridsize_2))
  (bind _returnvalue_2 (- _gridsize 1))
  (bind _returnvalue_3 (- _gridsize_3 1))
  (bind _returnvalue_4 (/ 1.0 _returnvalue))
  (bind _arrayelement (Utilities|Array|ReverseforEachLoop _spaceslist)
    (:LoopBody
      (Components|DestroyComponent _arrayelement))
    (:Completed
      (Utilities|Array|Clear _spaceslist)
      (bind _arrayelement_2 (Utilities|Array|ReverseforEachLoop _mesheslist)
        (:LoopBody
          (Components|DestroyComponent _arrayelement_2))
        (:Completed
          (Utilities|Array|Clear _mesheslist)
          (for _index (range 0 _returnvalue_2)
            (Variables|Default|SetY_Index _index)
            (for _index_2 (range 0 _returnvalue_2)
              (Variables|Default|SetX_index _index_2)
              (bind _returnvalue_5 (AddComponent|AddBoxComponent false (Math|Transform|MakeTransform (Math|Vector|MakeVector (* (Variables|Default|GetX_index) _mesh_size) (* (Variables|Default|GetY_Index) _mesh_size) 0.0) "0, 0, 0" "1.000000,1.000000,1.000000")))
              (Components|Box|SetBoxExtent _returnvalue_5 (Math|Conversions|ToVector(Float) (/ (Variables|Default|GetMesh_Size) 4.0)) true)
              (Utilities|Array|AddUnique (Variables|Default|GetSpaceslist) _returnvalue_5)
              (if (not (and (== (Variables|Default|GetY_Index) _returnvalue_3) (== _returnvalue_3 (Variables|Default|GetX_index))))
                (bind _returnvalue_6 (AddComponent|AddStaticMeshComponent false (Math|Transform|MakeTransform (Math|Vector|MakeVector (* (Variables|Default|GetX_index) _mesh_size_2) (* (Variables|Default|GetY_Index) _mesh_size_2) 0.0) "0, 0, 0" (Math|Conversions|ToVector(Float) (Variables|Default|Getsize)))))
                (Utilities|Array|AddUnique (Variables|Default|GetMesheslist) _returnvalue_6)
                (bind _returnvalue_7 (Rendering|Material|CreateDynamicMaterialInstance _returnvalue_6 0 "/Game/08Minigame/M_puzzle_material.M_puzzle_material" "None" :!class /Script/Engine.PrimitiveComponent))
                (Rendering|Material|SetTextureParameterValue _returnvalue_7 "PuzzleTexture" (Variables|Default|GetTexture))
                (Rendering|Material|SetVectorParameterValueonMaterials _returnvalue_6 "TextureOffset2D" (Math|Vector|MakeVector (* _returnvalue_4 (Variables|Default|GetX_index)) (* _returnvalue_4 (Variables|Default|GetY_Index)) _returnvalue)))))
          (return))))))

(fn ShufflePuzzle
  (bind _locations (LocalVariables|GetLocations))
  (bind _locations_2 (LocalVariables|GetLocations))
  (if (Variables|Default|Getshuffle?)
    (for _array_element (Variables|Default|GetSpaceslist)
      (Utilities|Array|Add _locations (Variables|/Script/Engine.SceneComponent|GetRelativeLocation _array_element)))
    (Utilities|Array|Shuffle _locations)
    (for _array_element_2 (Variables|Default|GetMesheslist)
      (Transformation|SetRelativeLocation _array_element_2 (Utilities|Array|Get(acopy) _locations_2) false false)
      (Utilities|Array|RemoveIndex _locations_2))
    (return)
    (else
      (return))))

(fn GetNeighbors
  (bind _outcomponents (Collision|SphereOverlapComponents (Transformation|GetWorldLocation (Variables|Default|GetClicked%20Mesh)) (Variables|Default|GetMesh_Size) (Utilities|Array|MakeArray "ObjectTypeQuery1" "ObjectTypeQuery2") "/Script/Engine.BoxComponent"))
  (return _outcomponents))