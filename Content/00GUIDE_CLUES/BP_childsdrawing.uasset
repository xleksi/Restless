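; BP_childsdrawing is an interactable child's drawing clue that opens a full-screen UI when the player interacts with it.
; Looking at it toggles a prompt widget, and a map outline event toggles custom depth on the note when the item ID matches.
; Interacting flags the character as viewing a widget, then creates WBP_childsdrawing if none exists, switches input to UI-only and plays a sound.
; It always reports that it cannot be picked up.
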(event `/Game/03Assets/BI_HighLightCommuncation.LookAtItem`
  (params (`?LookAt` :type Boolean))
  (`SceneComponent.SetVisibility` (`self.Widget`) `?LookAt` false)
  (set `self.?AbleToPickUp` `?LookAt`))

(event `/Game/03Assets/BI_HighLightCommuncation.OutlineOnMap`
  (params (`?Outline` :type Boolean) (NumberID :type "Float (double-precision)"))
  (if (== NumberID (`self.ItemID`))
    (`PrimitiveComponent.SetRenderCustomDepth` (`self.note`) `?Outline`)))

(event `/Game/03Assets/BI_HighLightCommuncation.InteractItem`
  (bind _asbp_third_person_character (cast `/Game/ThirdPerson/Blueprints/BP_ThirdPersonCharacter` (`GameplayStatics.GetPlayerCharacter` 0)))
  (set `/Game/ThirdPerson/Blueprints/BP_ThirdPersonCharacter.?LookingAtWidget` true _asbp_third_person_character)
  (set `PlayerController.bShowMouseCursor` false (`GameplayStatics.GetPlayerController` 0))
  (`self.ChildDrawing`
    (:`then`)
    (:`else`
      (`|ExecutionSequence`
        (:`then_0`
          ;[1 0.8805 0] Comment
          (bind _returnvalue (`|CreateWidget` "/Game/00GUIDE_CLUES/WBP_childsdrawing.WBP_childsdrawing_C"))
          (bind _output_get (set `self.ChildDrawing` _returnvalue))
          (`UserWidget.AddToViewport` _output_get 0)
          (`WidgetBlueprintLibrary.SetInputMode_UIOnlyEx` (`GameplayStatics.GetPlayerController` 0) (`self.ChildDrawing`)))
        (:`then_1`
          (`GameplayStatics.PlaySound2D` "/Game/00GUIDE_CLUES/pickupnote.pickupnote" 1.0 1.0 0.0 null null))))))

(fn `IsAbleToBePickedUp`
  (returns (`?AbleToPickUp` :type Boolean))
  (return false))

(fn `UserConstructionScript`)