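; Guide note pickup actor that shows a clue note on screen while the player stands inside its Box trigger.
; Player overlap plays a pickup sound, creates the WBP_guidenote_2 widget and adds it to the viewport.
; Ending any overlap, with no check for the player, plays a put-down sound and removes that widget.
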(event `self.Box.OnComponentBeginOverlap`
  (params (OverlappedComponent :type "PrimitiveComponent Object Reference") (OtherActor :type "Actor Object Reference") (OtherComp :type "PrimitiveComponent Object Reference") (OtherBodyIndex :type Integer) (bFromSweep :type Boolean) (SweepResult :type "HitResult Structure (by ref)"))
  (if (== OtherActor (`GameplayStatics.GetPlayerCharacter` 0))
    (`GameplayStatics.PlaySound2D` "/Game/00GUIDE_CLUES/pickupnote.pickupnote" 1.0 1.0 0.0 null null)
    (`self.pickup note`)))

(event `self.Box.OnComponentEndOverlap`
  (params (OverlappedComponent :type "PrimitiveComponent Object Reference") (OtherActor :type "Actor Object Reference") (OtherComp :type "PrimitiveComponent Object Reference") (OtherBodyIndex :type Integer))
  (`GameplayStatics.PlaySound2D` "/Game/04Sound/SoundPlaceholder/putdownnote.putdownnote" 1.0 1.0 0.0 null null)
  (`self.put down note`))

(event `pickup note`
  (bind _returnvalue (`|CreateWidget` "/Game/00GUIDE_CLUES/WBP_guidenote_2.WBP_guidenote_2_C"))
  (`UserWidget.AddToViewport` _returnvalue 0))

(event `put down note`
  (`Widget.RemoveFromParent` (stale `pickup note` _returnvalue)))

(fn `UserConstructionScript`)