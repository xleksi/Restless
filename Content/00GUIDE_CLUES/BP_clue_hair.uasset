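; BP_clue_hair is an interactable hair clue that the player can look at and inspect.
; Look-at events toggle its prompt widget and the pickup flag, which IsAbleToBePickedUp reports.
; An outline event toggles custom depth on the hair mesh when the given ID matches its ItemID.
; Interacting flags the character as viewing a widget, hides the cursor, and opens WBP_hair in UI-only input mode.
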(event `/Game/03Assets/BI_HighLightCommuncation.LookAtItem`
  (params (`?LookAt` :type Boolean))
  (`SceneComponent.SetVisibility` (`self.Widget`) `?LookAt` false)
  (set `self.?AbleToPickUp` `?LookAt`))

(event `/Game/03Assets/BI_HighLightCommuncation.OutlineOnMap`
  (params (`?Outline` :type Boolean) (NumberID :type "Float (double-precision)"))
  (if (== NumberID (`self.ItemID`))
    (`PrimitiveComponent.SetRenderCustomDepth` (`self.Hair`) `?Outline`)))

(event `/Game/03Assets/BI_HighLightCommuncation.InteractItem`
  (bind _asbp_third_person_character (cast `/Game/ThirdPerson/Blueprints/BP_ThirdPersonCharacter` (`GameplayStatics.GetPlayerCharacter` 0)))
  (set `/Game/ThirdPerson/Blueprints/BP_ThirdPersonCharacter.?LookingAtWidget` true _asbp_third_person_character)
  (set `PlayerController.bShowMouseCursor` false (`GameplayStatics.GetPlayerController` 0))
  ;[1 0.8805 0] Comment
  (bind _returnvalue (`|CreateWidget` "/Game/00GUIDE_CLUES/WBP_hair.WBP_hair_C"))
  (bind _output_get (set `self.HairWidget` _returnvalue))
  (`UserWidget.AddToViewport` _output_get 0)
  (`WidgetBlueprintLibrary.SetInputMode_UIOnlyEx` (`GameplayStatics.GetPlayerController` 0) (`self.HairWidget`)))

(fn `IsAbleToBePickedUp`
  (returns (`?AbleToPickUp` :type Boolean))
  (return (`self.?AbleToPickUp`)))

(fn `UserConstructionScript`)