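; Inventory component holding a fixed-capacity array of item slots, with BP_BaseItem marking empty ones.
; ProcessItem fills matching stacks up to their class-default limit, then empty slots, recursing on overflow.
; Adding a whole key or consuming any item messages every BP_DoorPlaceholder, and changes refresh the player's HUD.
; It also tracks two key part types in counts and lists, which CraftedKey removes in pairs.
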(event `self.ReceiveBeginPlay`
  (`KismetArrayLibrary.Array_Resize` (`self.Items`) (`self.Capacity`))
  (for (_ _array_index) (`self.Items`)
    (`KismetArrayLibrary.Array_Set` (`self.Items`) _array_index (make `/Game/06UI/Inventory/F_InventoryItem` "/Game/06UI/Inventory/Interactables/BP_BaseItem.BP_BaseItem_C" 0 self _array_index))))

(fn `AddItem`
  (params (ItemAdd :type "/Game/06UI/Inventory/F_InventoryItem Structure") (IndexLocation :type Integer))
  (returns (NewParam :type "/Game/06UI/Inventory/F_InventoryItem Structure"))
  (locals (LItem :type "/Game/06UI/Inventory/F_InventoryItem Structure") (LQuantity :type Integer :default 0) (AddItem :type "/Game/06UI/Inventory/F_InventoryItem Structure"))
  (bind ((`Item_12_5A8FA31948FEFCDF46485E91FCF07E3D` _item)) (break `/Game/06UI/Inventory/F_InventoryItem` (`local.AddItem`)))
  (bind _output (`|GetArrayItem` (`self.Items`) IndexLocation))
  (bind _output_get (set `local.LItem` ItemAdd))
  (bind ((`Item_12_5A8FA31948FEFCDF46485E91FCF07E3D` _item_2) (`Quantity_4_B7CF37DE41ED29050EA9B48C4313AC88` _quantity)) (break `/Game/06UI/Inventory/F_InventoryItem` _output_get))
  (bind _returnvalue (+ (`.Quantity_4_B7CF37DE41ED29050EA9B48C4313AC88` (break `/Game/06UI/Inventory/F_InventoryItem` _output)) _quantity))
  (bind _stacksize (defaults `Object` _item_2))
  (set `local.LQuantity` (- _returnvalue _stacksize))
  (bind _structout (setmembers `/Game/06UI/Inventory/F_InventoryItem` :`StructRef` _output :`Item` _item_2 :`Quantity` (`KismetMathLibrary.Clamp` _returnvalue 0 _stacksize) :`OwningInventory` self :`IndexLocation` (`local.IndexLocation`)))
  (set `local.AddItem` _structout)
  ;[0.3021 0.3021 0.3021] needed here because of locationchange happens here
  (if (== (`.Item_12_5A8FA31948FEFCDF46485E91FCF07E3D` (break `/Game/06UI/Inventory/F_InventoryItem` (`local.AddItem`))) "/Game/06UI/Inventory/Interactables/Keys/BP_WholeKey.BP_WholeKey_C")
    (bind _outactors (`GameplayStatics.GetAllActorsOfClass` "/Game/06UI/Inventory/Interactables/Door/BP_DoorPlaceholder.BP_DoorPlaceholder_C"))
    (for _array_element _outactors
      (message `/Game/06UI/Inventory/Interfaces/BI_InteractDoor.getKey` _array_element (`local.AddItem`))))
  ;[0.9652 1 0] Add nodes for crafting
  (if (or (== _item "/Game/06UI/Inventory/Interactables/Keys/BP_KeyPart_01.BP_KeyPart_01_C") (== _item "/Game/06UI/Inventory/Interactables/Keys/BP_KeyPart_02.BP_KeyPart_02_C"))
    (if (== (`.Item_12_5A8FA31948FEFCDF46485E91FCF07E3D` (break `/Game/06UI/Inventory/F_InventoryItem` (`local.AddItem`))) "/Game/06UI/Inventory/Interactables/Keys/BP_KeyPart_01.BP_KeyPart_01_C")
      (`/Engine/EditorBlueprintResources/StandardMacros.IncrementInt` (`self.KeyPart1Count`)
        (:`  `
          (`KismetArrayLibrary.Array_Add` (`self.KeyPart1List`) (`local.AddItem`))))
      (else
        (`/Engine/EditorBlueprintResources/StandardMacros.IncrementInt` (`self.KeyPart2Count`)
          (:`  `
            (`KismetArrayLibrary.Array_Add` (`self.KeyPart2List`) (`local.AddItem`)))))))
  (bind _structout_2 (setmembers `/Game/06UI/Inventory/F_InventoryItem` :`StructRef` (`local.LItem`) :`Quantity` (`local.LQuantity`)))
  (`self.UpdateInventoryHud`)
  (return _structout_2))

(fn `ConsumeItem`
  (params (Item :type "/Game/06UI/Inventory/F_InventoryItem Structure"))
  (bind ((`Quantity_4_B7CF37DE41ED29050EA9B48C4313AC88` _quantity) (`IndexLocation_11_B12A17D04100958D495318B3BD5D709B` _indexlocation)) (break `/Game/06UI/Inventory/F_InventoryItem` Item))
  (set `self.Item` Item)
  (bind _result (`/Engine/EditorBlueprintResources/StandardMacros.DecrementInt` _quantity)
    (:`  `
      (if (<= _result 0)
        (`|ExecutionSequence`
          (:`then_0`
            (`self.RemoveItem` (`self.Item`))
            (`KismetSystemLibrary.PrintString` "removed"))
          (:`then_1`
            (`self.UpdateInventoryHUD` :!label _label)
            (bind _outactors (`GameplayStatics.GetAllActorsOfClass` "/Game/06UI/Inventory/Interactables/Door/BP_DoorPlaceholder.BP_DoorPlaceholder_C"))
            (for _array_element _outactors
              (message `/Game/06UI/Inventory/Interfaces/BI_InteractDoor.KeyUsed` _array_element (struct)))
            (return)))
        (else
          (setmembers `/Game/06UI/Inventory/F_InventoryItem` :`StructRef` (`|GetArrayItem` (`self.Items`) _indexlocation))
          (goto _label))))))

(fn `CraftedKey`
  (`/Engine/EditorBlueprintResources/StandardMacros.DecrementInt` (`self.KeyPart1Count`)
    (:`  `
      (`/Engine/EditorBlueprintResources/StandardMacros.DecrementInt` (`self.KeyPart2Count`)
        (:`  `
          (`|ExecutionSequence`
            (:`then_0`
              (`self.RemoveItem` (`|GetArrayItem` (`self.KeyPart1List`) (`self.Counter`)))
              (`KismetSystemLibrary.PrintString` "remove1"))
            (:`then_1`
              (`self.RemoveItem` (`|GetArrayItem` (`self.KeyPart2List`) (`self.Counter`)))
              (`KismetSystemLibrary.PrintString` "remove2"))
            (:`then_2`
              (`self.UpdateInventoryHUD`))
            (:`then_3`
              (`/Engine/EditorBlueprintResources/StandardMacros.IncrementInt` (`self.Counter`)))))))))

(fn `FindAvailableLocation`
  (params (Item :type "/Game/06UI/Inventory/F_InventoryItem Structure"))
  (returns (IndexLocation :type Integer))
  (locals (LIndexLocation :type Integer :default -1))
  (for (_array_element _array_index) (`self.Items`)
    (bind ((`Item_12_5A8FA31948FEFCDF46485E91FCF07E3D` _item) (`Quantity_4_B7CF37DE41ED29050EA9B48C4313AC88` _quantity)) (break `/Game/06UI/Inventory/F_InventoryItem` _array_element))
    (if (and (== Item_Item_12_5A8FA31948FEFCDF46485E91FCF07E3D _item) (< _quantity (defaults `Object` _item)))
      (set `local.LIndexLocation` _array_index)
      (break)))
  (if (< (`local.LIndexLocation`) 0)
    (for (_array_element_2 _array_index_2) (`self.Items`)
      (if (== (`.Item_12_5A8FA31948FEFCDF46485E91FCF07E3D` (break `/Game/06UI/Inventory/F_InventoryItem` _array_element_2)) "/Game/06UI/Inventory/Interactables/BP_BaseItem.BP_BaseItem_C")
        (set `local.LIndexLocation` _array_index_2)
        (break)))
    (return (`local.LIndexLocation`))
    (else
      (return (`local.LIndexLocation`)))))

(fn `ProcessItem`
  (params (Item :type "/Game/06UI/Inventory/F_InventoryItem Structure"))
  (returns (Quantity :type Integer))
  (bind _indexlocation (`self.FindAvailableLocation` Item))
  (if (>= _indexlocation 0)
    (bind _newparam (`self.AddItem` (`local.Item`) _indexlocation))
    (bind ((`Quantity_4_B7CF37DE41ED29050EA9B48C4313AC88` _quantity)) (break `/Game/06UI/Inventory/F_InventoryItem` _newparam))
    (if (> _quantity 0)
      (bind _quantity_2 (`self.ProcessItem` _newparam))
      (return _quantity_2)
      (else
        (return _quantity)))
    (else
      (`KismetSystemLibrary.PrintString` "Inventory Full")
      (return (`.Quantity_4_B7CF37DE41ED29050EA9B48C4313AC88` (break `/Game/06UI/Inventory/F_InventoryItem` (`local.Item`)))))))

(fn `RemoveItem`
  (params (Items :type "/Game/06UI/Inventory/F_InventoryItem Structure"))
  (returns (bSuccess :type Boolean))
  (bind ((`IndexLocation_11_B12A17D04100958D495318B3BD5D709B` _indexlocation)) (break `/Game/06UI/Inventory/F_InventoryItem` Items))
  (setmembers `/Game/06UI/Inventory/F_InventoryItem` :`StructRef` (`|GetArrayItem` (`self.Items`) _indexlocation) :`Item` "/Game/06UI/Inventory/Interactables/BP_BaseItem.BP_BaseItem_C" :`Quantity` 0 :`OwningInventory` self :`IndexLocation` _indexlocation)
  (return true))

(fn `UpdateInventoryHUD`
  (message `/Game/06UI/Inventory/Interfaces/BI_InteractHUB.UpdateInventoryHUD` (`GameplayStatics.GetPlayerCharacter` 0) self)
  (return))

(fn `UpdateKeyParts`
  (returns (NewParam :type Integer) (NewParam1 :type Integer))
  (return (`self.KeyPart1Count`) (`self.KeyPart2Count`)))