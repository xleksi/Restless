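; Inventory component that stores general items and keys for its owning BP_ThirdPersonCharacter.
; Adding an item or key appends it to its own array, prints it, then casts the owner to update that character's InventoryWidget.
; RemoveKey takes no argument: it removes an empty value from the key array, prints a debug message and calls the widget's RemoveKey.
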(fn `AddItemtoInventory`
  (params (NewItem :type "String (by ref)"))
  (`KismetArrayLibrary.Array_Add` (`self.inventory`) NewItem)
  (`KismetSystemLibrary.PrintString` NewItem)
  (bind _asbp_third_person_character (cast `/Game/ThirdPerson/Blueprints/BP_ThirdPersonCharacter` (`self.GetOwner`)))
  (`/Game/06UI/Inventory/WBP_Inventory.Add Item to List Ui` (`/Game/ThirdPerson/Blueprints/BP_ThirdPersonCharacter.Inventory Widget` _asbp_third_person_character) NewItem))

(fn `AddKeytoInventory`
  (params (Item :type String))
  (`KismetArrayLibrary.Array_Add` (`self.KEyInventor`) Item)
  (`KismetSystemLibrary.PrintString` Item)
  (bind _asbp_third_person_character (cast `/Game/ThirdPerson/Blueprints/BP_ThirdPersonCharacter` (`self.GetOwner`)))
  (`/Game/06UI/Inventory/WBP_Inventory.Add Key` (`/Game/ThirdPerson/Blueprints/BP_ThirdPersonCharacter.Inventory Widget` _asbp_third_person_character) Item))

(fn `RemoveKey`
  (`KismetArrayLibrary.Array_RemoveItem` (`self.KEyInventor`))
  (`KismetSystemLibrary.PrintString` "Hello")
  (bind _asbp_third_person_character (cast `/Game/ThirdPerson/Blueprints/BP_ThirdPersonCharacter` (`self.GetOwner`)))
  (`/Game/06UI/Inventory/WBP_Inventory.Remove Key` (`/Game/ThirdPerson/Blueprints/BP_ThirdPersonCharacter.Inventory Widget` _asbp_third_person_character)))