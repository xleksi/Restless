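; Interactable small bookshelf Blueprint with a right door that the player can swing open and closed.
; LookatObjectMesh tracks the looked-at mesh, toggling a custom-depth outline and the door's prompt widget, while skipping the middle shelf mesh.
; Interactwith calls OpenCloseStuff, which picks the target yaw from the door's current rotation and lerps it with a timeline.
; A Wait flag blocks new interactions until the animation finishes.
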(event `self.ReceiveBeginPlay`
  (set `self.MeshArray` (`|MakeArray` (`self.Door_Right`)))
  (set `self.WidgetArray` (`|MakeArray` (`self.WidgetDoor_Right`))))

(event `/Game/ThirdPerson/Blueprints/BI_InteractableObjects.LookAtObjectMesh`
  (params (HitComponent :type "ActorComponent Object Reference") (`?LookAt` :type Boolean))
  ;[1 0.1086 0.7114] Mesh checking  -> outline already there
  (bind _output_get (set `self.?LookAt` `?LookAt`))
  (if _output_get
    (bind _asstatic_mesh_component (cast `StaticMeshComponent` HitComponent))
    (set `self.LookAtMesh` _asstatic_mesh_component)
    (if (== (`self.CurrentMesh`) (`self.LookAtMesh`))
      (`self.InteractMesh` true)
      (else
        (`/Engine/EditorBlueprintResources/StandardMacros.IsValid` (`self.CurrentMesh`)
          (:`Is Valid`
            (for _array_element (`self.MeshArray`)
              (`PrimitiveComponent.SetRenderCustomDepth` _array_element false)
              (for _array_element_2 (`self.WidgetArray`)
                (`SceneComponent.SetVisibility` _array_element_2 false false))
              (set `self.CurrentMesh` (`self.LookAtMesh`))
              (`self.InteractMesh` true)))
          (:`Is Not Valid`
            (set `self.CurrentMesh` (`self.LookAtMesh`))
            (`self.InteractMesh` true)))))
    (else
      (for _array_element_3 (`self.MeshArray`)
        (`PrimitiveComponent.SetRenderCustomDepth` _array_element_3 false))
      (for _array_element_4 (`self.WidgetArray`)
        (`SceneComponent.SetVisibility` _array_element_4 false false)))))

(event `/Game/ThirdPerson/Blueprints/BI_InteractableObjects.InteractWith`
  ;[1 1 1] Comment
  (if (`self.?LookAt`)
    (if (not (`self.?Wait`))
      (`self.Open/CloseStuff`))))

(event `AnimateDoorRight`
  ;[0.4055 1 0.5729] Opening Door Right
  (bind (_direction _drawer) (`Timeline|Timeline` :!via `PlayFromStart`)
    (:`Update`
      (`SceneComponent.K2_SetRelativeRotation` (`self.Door_Right`) (`KismetMathLibrary.RLerp` (`self.StartRotation`) (`self.EndRottation`) _drawer) false false))
    (:`Finished`
      (set `self.?Wait` false))))

(fn `InteractDoorRight`
  (bind (_relativerotation_roll _relativerotation_pitch _relativerotation_yaw) (`KismetMathLibrary.BreakRotator` (`SceneComponent.RelativeRotation` (`self.Door_Right`))))
  (bind (_relativerotation_roll_2 _relativerotation_pitch_2 _relativerotation_yaw_2) (`KismetMathLibrary.BreakRotator` (`SceneComponent.RelativeRotation` (`self.Door_Right`))))
  (bind (_relativerotation_roll_3 _relativerotation_pitch_3 _relativerotation_yaw_3) (`KismetMathLibrary.BreakRotator` (`SceneComponent.RelativeRotation` (`self.Door_Right`))))
  (if (not (<= _relativerotation_yaw_2 -109.0))
    (set `self.StartRotation` (`KismetMathLibrary.MakeRotator` _relativerotation_roll_3 _relativerotation_pitch_3 _relativerotation_yaw_3))
    (set `self.EndRottation` (`KismetMathLibrary.MakeRotator` _relativerotation_roll_3 _relativerotation_pitch_3 -110.0))
    (else
      (set `self.StartRotation` (`KismetMathLibrary.MakeRotator` _relativerotation_roll _relativerotation_pitch _relativerotation_yaw))
      (set `self.EndRottation` (`KismetMathLibrary.MakeRotator` _relativerotation_roll _relativerotation_pitch))))
  (`self.AnimateDoorRight`))

(fn `InteractMesh`
  (params (`?Outline` :type Boolean))
  (set `self.? Outline` `?Outline`)
  (if (not (== (`self.Bookshelvemiddleempty`) (`self.CurrentMesh`)))
    (`PrimitiveComponent.SetRenderCustomDepth` (`self.CurrentMesh`) (`self.? Outline`))
    (if (== (`self.Door_Right`) (`self.CurrentMesh`))
      (`SceneComponent.SetVisibility` (`self.WidgetDoor_Right`) (`self.? Outline`) false))))

(fn `Open/CloseStuff`
  (if (`self.?Wait`)
    _
    (elif (== (`self.CurrentMesh`) (`self.Door_Right`))
      (set `self.?Wait` true)
      (`self.InteractDoorRight`))))

(fn `UserConstructionScript`)