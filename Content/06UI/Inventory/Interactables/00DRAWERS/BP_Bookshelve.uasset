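; Interactable bookshelf whose left and right doors the player can open and close individually.
; While something overlaps BorderBox, look-at events set the targeted mesh as current, highlighting doors with a custom-depth outline and showing their prompt widget.
; Interacting toggles that door's yaw between closed and about 110 degrees outward through a timeline rotation lerp.
; A Wait flag blocks further input until the animation finishes.
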(event `self.ReceiveBeginPlay`
  (set `self.MeshArray` (`|MakeArray` (`self.Door_Right`) (`self.Door_Left`)))
  (set `self.WidgetArray` (`|MakeArray` (`self.WidgetDoor_Right`) (`self.WidgetDoor_Left`))))

(event `/Game/ThirdPerson/Blueprints/BI_InteractableObjects.LookAtObjectMesh`
  (params (HitComponent :type "ActorComponent Object Reference") (`?LookAt` :type Boolean))
  ;[1 0.1086 0.7114] Mesh checking  -> outline already there
  (bind _output_get (set `self.?LookAt` `?LookAt`))
  (if (`self.?Wait`)
    _
    (elif (`self.?NearObject`)
      (if _output_get
        (bind _asstatic_mesh_component (cast `StaticMeshComponent` HitComponent))
        (set `self.LookAtMesh` _asstatic_mesh_component)
        (if (== (`self.CurrentMesh`) (`self.LookAtMesh`))
          (`self.InteractMesh` true)
          (else
            (`/Engine/EditorBlueprintResources/StandardMacros.IsValid` (`self.CurrentMesh`)
              (:`Is Valid`
                (for _array_element (`self.MeshArray`)
                  (`PrimitiveComponent.SetRenderCustomDepth` _array_element false)
                  (for _array_element_2 (`self.WidgetArray`)
                    (`SceneComponent.SetVisibility` _array_element_2 false false))
                  (set `self.CurrentMesh` (`self.LookAtMesh`))
                  (`self.InteractMesh` true)))
              (:`Is Not Valid`
                (set `self.CurrentMesh` (`self.LookAtMesh`))
                (`self.InteractMesh` true)))))
        (else
          (for _array_element_3 (`self.MeshArray`)
            (`PrimitiveComponent.SetRenderCustomDepth` _array_element_3 false))
          (for _array_element_4 (`self.WidgetArray`)
            (`SceneComponent.SetVisibility` _array_element_4 false false)))))))

(event `/Game/ThirdPerson/Blueprints/BI_InteractableObjects.InteractWith`
  ;[1 1 1] Comment
  (if (`self.?LookAt`)
    (if (not (`self.?Wait`))
      (`self.Open/CloseStuff`))))

(event `AnimateDoorRight`
  ;[0.4055 1 0.5729] Opening Door Right
  (bind (_direction _drawer) (`Timeline|Timeline` :!via `PlayFromStart`)
    (:`Update`
      (`SceneComponent.K2_SetRelativeRotation` (`self.Door_Right`) (`KismetMathLibrary.RLerp` (`self.StartRotation`) (`self.EndRottation`) _drawer) false false))
    (:`Finished`
      (set `self.?Wait` false))))

(event `self.BorderBox.OnComponentBeginOverlap`
  (params (OverlappedComponent :type "PrimitiveComponent Object Reference") (OtherActor :type "Actor Object Reference") (OtherComp :type "PrimitiveComponent Object Reference") (OtherBodyIndex :type Integer) (bFromSweep :type Boolean) (SweepResult :type "HitResult Structure (by ref)"))
  (set `self.?NearObject` true))

(event `self.BorderBox.OnComponentEndOverlap`
  (params (OverlappedComponent :type "PrimitiveComponent Object Reference") (OtherActor :type "Actor Object Reference") (OtherComp :type "PrimitiveComponent Object Reference") (OtherBodyIndex :type Integer))
  (set `self.?NearObject` false)
  (for _array_element (`self.MeshArray`)
    (`PrimitiveComponent.SetRenderCustomDepth` _array_element false))
  (for _array_element_2 (`self.WidgetArray`)
    (`SceneComponent.SetVisibility` _array_element_2 false false)))

(event `AnimateDoorLeft`
  ;[0.4055 1 0.5729] Opening Door Left
  (bind (_direction _drawer) (`Timeline|Timeline_0` :!via `PlayFromStart`)
    (:`Update`
      (`SceneComponent.K2_SetRelativeRotation` (`self.Door_Left`) (`KismetMathLibrary.RLerp` (`self.StartRotation`) (`self.EndRottation`) _drawer) false false))
    (:`Finished`
      (set `self.?Wait` false))))

(fn `InteractDoorLeft`
  (bind (_relativerotation_roll _relativerotation_pitch _relativerotation_yaw) (`KismetMathLibrary.BreakRotator` (`SceneComponent.RelativeRotation` (`self.Door_Left`))))
  (bind (_relativerotation_roll_2 _relativerotation_pitch_2 _relativerotation_yaw_2) (`KismetMathLibrary.BreakRotator` (`SceneComponent.RelativeRotation` (`self.Door_Left`))))
  (bind (_relativerotation_roll_3 _relativerotation_pitch_3 _relativerotation_yaw_3) (`KismetMathLibrary.BreakRotator` (`SceneComponent.RelativeRotation` (`self.Door_Left`))))
  (if (not (>= _relativerotation_yaw_2 109.0))
    (set `self.StartRotation` (`KismetMathLibrary.MakeRotator` _relativerotation_roll_3 _relativerotation_pitch_3 _relativerotation_yaw_3))
    (set `self.EndRottation` (`KismetMathLibrary.MakeRotator` _relativerotation_roll_3 _relativerotation_pitch_3 110.0))
    (else
      (set `self.StartRotation` (`KismetMathLibrary.MakeRotator` _relativerotation_roll _relativerotation_pitch _relativerotation_yaw))
      (set `self.EndRottation` (`KismetMathLibrary.MakeRotator` _relativerotation_roll _relativerotation_pitch))))
  (`self.AnimateDoorLeft`))

(fn `InteractDoorRight`
  (bind (_relativerotation_roll _relativerotation_pitch _relativerotation_yaw) (`KismetMathLibrary.BreakRotator` (`SceneComponent.RelativeRotation` (`self.Door_Right`))))
  (bind (_relativerotation_roll_2 _relativerotation_pitch_2 _relativerotation_yaw_2) (`KismetMathLibrary.BreakRotator` (`SceneComponent.RelativeRotation` (`self.Door_Right`))))
  (bind (_relativerotation_roll_3 _relativerotation_pitch_3 _relativerotation_yaw_3) (`KismetMathLibrary.BreakRotator` (`SceneComponent.RelativeRotation` (`self.Door_Right`))))
  (if (not (<= _relativerotation_yaw_2 -109.0))
    (set `self.StartRotation` (`KismetMathLibrary.MakeRotator` _relativerotation_roll_3 _relativerotation_pitch_3 _relativerotation_yaw_3))
    (set `self.EndRottation` (`KismetMathLibrary.MakeRotator` _relativerotation_roll_3 _relativerotation_pitch_3 -110.0))
    (else
      (set `self.StartRotation` (`KismetMathLibrary.MakeRotator` _relativerotation_roll _relativerotation_pitch _relativerotation_yaw))
      (set `self.EndRottation` (`KismetMathLibrary.MakeRotator` _relativerotation_roll _relativerotation_pitch))))
  (`self.AnimateDoorRight`))

(fn `InteractMesh`
  (params (`?Outline` :type Boolean))
  (set `self.? Outline` `?Outline`)
  (if (not (== (`self.Bookshelvemiddleempty`) (`self.CurrentMesh`)))
    (`PrimitiveComponent.SetRenderCustomDepth` (`self.CurrentMesh`) (`self.? Outline`))
    (if (== (`self.Door_Left`) (`self.CurrentMesh`))
      (`SceneComponent.SetVisibility` (`self.WidgetDoor_Left`) (`self.? Outline`) false)
      (elif (== (`self.Door_Right`) (`self.CurrentMesh`))
        (`SceneComponent.SetVisibility` (`self.WidgetDoor_Right`) (`self.? Outline`) false)))))

(fn `Open/CloseStuff`
  (if (`self.?Wait`)
    _
    (elif (== (`self.CurrentMesh`) (`self.Door_Right`))
      (set `self.?Wait` true)
      (`self.InteractDoorRight`)
      (elif (== (`self.CurrentMesh`) (`self.Door_Left`))
        (set `self.?Wait` true)
        (`self.InteractDoorLeft`)))))

(fn `UserConstructionScript`)