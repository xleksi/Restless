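; Interactable kitchen cupboard with four doors and two drawers that open and close individually.
; Looking at a part highlights it via custom depth and shows its widget, matched by index in parallel mesh and widget arrays.
; Interacting picks drawer slide or door swing, choosing direction from the part's current transform.
; Timelines lerp the motion while a Wait flag blocks input; both door sides use AnimateDoorLeft, leaving AnimateDoorRight uncalled.
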(event `self.ReceiveBeginPlay`
  ;[0.08854 0.08854 0.08854] arrays for easy outline removale
  (set `self.Mesh Array` (`|MakeArray` (`self.DoorLeftBottom`) (`self.DrawerRight`) (`self.DrawerLeft`) (`self.DoorRightTop`) (`self.DoorLeftTop`) (`self.DoorRightBottom`)))
  (set `self.Widget Array` (`|MakeArray` (`self.WidgetDoorLeftBottom`) (`self.WidgetDrawerRight`) (`self.WidgetDrawerLeft`) (`self.WidgetDoorRightTop`) (`self.WidgetDoorLeftTop`) (`self.WidgetDoorRightBottom`))))

(event `/Game/ThirdPerson/Blueprints/BI_InteractableObjects.LookAtObjectMesh`
  (params (HitComponent :type "ActorComponent Object Reference") (`?LookAt` :type Boolean))
  ;[1 0.1086 0.7114] Mesh checking  -> outline already there
  (if (not (`self.?Wait`))
    (bind _output_get (set `self.? Look At` `?LookAt`))
    (if _output_get
      (bind _asstatic_mesh_component (cast `StaticMeshComponent` HitComponent))
      (set `self.LookAtMesh` _asstatic_mesh_component)
      (if (== (`self.CurrentMesh`) (`self.LookAtMesh`))
        (`self.InteractMesh` true)
        (else
          (`/Engine/EditorBlueprintResources/StandardMacros.IsValid` (`self.CurrentMesh`)
            (:`Is Valid`
              (for _array_element (`self.Mesh Array`)
                (`PrimitiveComponent.SetRenderCustomDepth` _array_element false))
              (for _array_element_2 (`self.Widget Array`)
                (`SceneComponent.SetVisibility` _array_element_2 false false))
              (set `self.CurrentMesh` (`self.LookAtMesh`))
              (`self.InteractMesh` true))
            (:`Is Not Valid`
              (set `self.CurrentMesh` (`self.LookAtMesh`))
              (`self.InteractMesh` true)))))
      (else
        (for _array_element_3 (`self.Mesh Array`)
          (`PrimitiveComponent.SetRenderCustomDepth` _array_element_3 false))
        (for _array_element_4 (`self.Widget Array`)
          (`SceneComponent.SetVisibility` _array_element_4 false false))))))

(event `/Game/ThirdPerson/Blueprints/BI_InteractableObjects.InteractWith`
  ;[1 1 1] Comment
  (if (`self.? Look At`)
    (if (not (`self.?Wait`))
      (`self.Open/Close Stuff`))))

(event `DrawerAnimate`
  ;[0.4055 1 0.5729] Opening Drawer Right
  (bind (_direction _drawer) (`Timeline|Timeline` :!via `PlayFromStart`)
    (:`Update`
      (`SceneComponent.K2_SetRelativeLocation` (`self.CurrentMesh`) (`KismetMathLibrary.VLerp` (`self.StartLocation`) (`self.EndLocation`) _drawer) false false))
    (:`Finished`
      (set `self.?Wait` false))))

(event `AnimateDoorRight`
  ;[0.4055 1 0.5729] Opening Door Right
  (bind (_direction _drawer) (`Timeline|Timeline_0` :!via `PlayFromStart`)
    (:`Update`
      (`SceneComponent.K2_SetRelativeRotation` (`self.CurrentMesh`) (`KismetMathLibrary.RLerp` (`self.StartRotation`) (`self.EndRottation`) _drawer) false false))
    (:`Finished`
      (set `self.?Wait` false))))

(event `AnimateDoorLeft`
  ;[0.4055 1 0.5729] Opening Door Left
  (bind (_direction _drawer) (`Timeline|Timeline_1` :!via `PlayFromStart`)
    (:`Update`
      (`SceneComponent.K2_SetRelativeRotation` (`self.CurrentMesh`) (`KismetMathLibrary.RLerp` (`self.StartRotation`) (`self.EndRottation`) _drawer) false false))
    (:`Finished`
      (set `self.?Wait` false))))

(fn `Interact Drawer`
  (bind _relativelocation_x (`KismetMathLibrary.BreakVector` (`SceneComponent.RelativeLocation` (`self.CurrentMesh`))))
  (bind (_relativelocation_x_2 _relativelocation_y _relativelocation_z) (`KismetMathLibrary.BreakVector` (`SceneComponent.RelativeLocation` (`self.CurrentMesh`))))
  (bind (_relativelocation_x_3 _relativelocation_y_2 _relativelocation_z_2) (`KismetMathLibrary.BreakVector` (`SceneComponent.RelativeLocation` (`self.CurrentMesh`))))
  (if (not (>= _relativelocation_x 2.0))
    (set `self.StartLocation` (`KismetMathLibrary.MakeVector` _relativelocation_x_3 _relativelocation_y_2 _relativelocation_z_2))
    (set `self.EndLocation` (`KismetMathLibrary.MakeVector` (`self.EndDrawer`) _relativelocation_y_2 _relativelocation_z_2))
    (else
      (set `self.StartLocation` (`KismetMathLibrary.MakeVector` _relativelocation_x_2 _relativelocation_y _relativelocation_z))
      (set `self.EndLocation` (`KismetMathLibrary.MakeVector` (`self.StartDrawer`) _relativelocation_y _relativelocation_z))))
  (`self.DrawerAnimate`))

(fn `InteractDoorLeft`
  (bind (_relativerotation_roll _relativerotation_pitch _relativerotation_yaw) (`KismetMathLibrary.BreakRotator` (`SceneComponent.RelativeRotation` (`self.CurrentMesh`))))
  (bind (_relativerotation_roll_2 _relativerotation_pitch_2 _relativerotation_yaw_2) (`KismetMathLibrary.BreakRotator` (`SceneComponent.RelativeRotation` (`self.CurrentMesh`))))
  (bind (_relativerotation_roll_3 _relativerotation_pitch_3 _relativerotation_yaw_3) (`KismetMathLibrary.BreakRotator` (`SceneComponent.RelativeRotation` (`self.CurrentMesh`))))
  (if (not (>= _relativerotation_yaw_2 109.0))
    (set `self.StartRotation` (`KismetMathLibrary.MakeRotator` _relativerotation_roll_3 _relativerotation_pitch_3 _relativerotation_yaw_3))
    (set `self.EndRottation` (`KismetMathLibrary.MakeRotator` _relativerotation_roll_3 _relativerotation_pitch_3 110.0))
    (`self.AnimateDoorLeft`)
    (else
      (set `self.StartRotation` (`KismetMathLibrary.MakeRotator` _relativerotation_roll _relativerotation_pitch _relativerotation_yaw))
      (set `self.EndRottation` (`KismetMathLibrary.MakeRotator` _relativerotation_roll _relativerotation_pitch))
      (`self.AnimateDoorLeft`))))

(fn `InteractDoorRight`
  (bind (_relativerotation_roll _relativerotation_pitch _relativerotation_yaw) (`KismetMathLibrary.BreakRotator` (`SceneComponent.RelativeRotation` (`self.CurrentMesh`))))
  (bind (_relativerotation_roll_2 _relativerotation_pitch_2 _relativerotation_yaw_2) (`KismetMathLibrary.BreakRotator` (`SceneComponent.RelativeRotation` (`self.CurrentMesh`))))
  (bind (_relativerotation_roll_3 _relativerotation_pitch_3 _relativerotation_yaw_3) (`KismetMathLibrary.BreakRotator` (`SceneComponent.RelativeRotation` (`self.CurrentMesh`))))
  (if (not (<= _relativerotation_yaw_2 -109.0))
    (set `self.StartRotation` (`KismetMathLibrary.MakeRotator` _relativerotation_roll_3 _relativerotation_pitch_3 _relativerotation_yaw_3))
    (set `self.EndRottation` (`KismetMathLibrary.MakeRotator` _relativerotation_roll_3 _relativerotation_pitch_3 -110.0))
    (else
      (set `self.StartRotation` (`KismetMathLibrary.MakeRotator` _relativerotation_roll _relativerotation_pitch _relativerotation_yaw))
      (set `self.EndRottation` (`KismetMathLibrary.MakeRotator` _relativerotation_roll _relativerotation_pitch))))
  (`self.AnimateDoorLeft`))

(fn `InteractMesh`
  (params (`Outline?` :type Boolean))
  (set `self.Outline?` `Outline?`)
  (if (not (== (`self.Base`) (`self.CurrentMesh`)))
    (`PrimitiveComponent.SetRenderCustomDepth` (`self.CurrentMesh`) (`local.Outline?`))
    (`SceneComponent.SetVisibility` (`|GetArrayItem` (`self.Widget Array`) (`KismetArrayLibrary.Array_Find` (`self.Mesh Array`) (`self.CurrentMesh`))) true false)))

(fn `Open/Close Stuff`
  (if (not (`self.?Wait`))
    (set `self.?Wait` true)
    (if (or (== (`self.DrawerRight`) (`self.CurrentMesh`)) (== (`self.DrawerLeft`) (`self.CurrentMesh`)))
      (`self.Interact Drawer`)
      (elif (or (== (`self.DoorLeftBottom`) (`self.CurrentMesh`)) (== (`self.DoorLeftTop`) (`self.CurrentMesh`)))
        (`self.InteractDoorLeft`)
        (elif (or (== (`self.DoorRightTop`) (`self.CurrentMesh`)) (== (`self.DoorRightBottom`) (`self.CurrentMesh`)))
          (`self.InteractDoorRight`))))))

(fn `UserConstructionScript`)