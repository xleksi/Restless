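; Interactable nightstand cabinet with a sliding drawer and a hinged door, each opened or closed separately.
; Look-at events track the targeted mesh, toggling its custom-depth outline and prompt widget, with arrays used to clear previous highlights.
; Interaction runs timelines that lerp drawer location or door yaw, choosing direction from the part's current transform.
; A shared Wait flag blocks further interaction until the animation finishes.
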(event `self.ReceiveBeginPlay`
  ;[0.08854 0.08854 0.08854] arrays for easy outline removale
  (set `self.Mesh Array` (`|MakeArray` (`self.Mesh_Nightstand_Drawer`) (`self.Mesh_Nightstand_Door`)))
  (set `self.Widget Array` (`|MakeArray` (`self.DoorRight`) (`self.DrawerLeft`))))

(event `/Game/ThirdPerson/Blueprints/BI_InteractableObjects.LookAtObjectMesh`
  (params (HitComponent :type "ActorComponent Object Reference") (`?LookAt` :type Boolean))
  ;[1 0.1086 0.7114] Mesh checking  -> outline already there
  (bind _output_get (set `self.? Look At` `?LookAt`))
  (if _output_get
    (bind _asstatic_mesh_component (cast `StaticMeshComponent` HitComponent)
      (:`then`
        (set `self.LookAtMesh` _asstatic_mesh_component)
        (if (== (`self.CurrentMesh`) (`self.LookAtMesh`))
          (`self.InteractMesh` true)
          (else
            (`/Engine/EditorBlueprintResources/StandardMacros.IsValid` (`self.CurrentMesh`)
              (:`Is Valid`
                (for _array_element (`self.Mesh Array`)
                  (`PrimitiveComponent.SetRenderCustomDepth` _array_element false))
                (for _array_element_2 (`self.Widget Array`)
                  (`SceneComponent.SetVisibility` _array_element_2 false false))
                (set `self.CurrentMesh` (`self.LookAtMesh`))
                (`self.InteractMesh` true))
              (:`Is Not Valid`
                (set `self.CurrentMesh` (`self.LookAtMesh`))
                (`self.InteractMesh` true))))))
      (:`CastFailed`
        (`KismetSystemLibrary.PrintString` "cast faild object")))
    (else
      (for _array_element_3 (`self.Mesh Array`)
        (`PrimitiveComponent.SetRenderCustomDepth` _array_element_3 false))
      (for _array_element_4 (`self.Widget Array`)
        (`SceneComponent.SetVisibility` _array_element_4 false false)))))

(event `/Game/ThirdPerson/Blueprints/BI_InteractableObjects.InteractWith`
  ;[1 1 1] Comment
  (if (`self.? Look At`)
    (if (not (`self.?Wait`))
      (`self.Open/Close Stuff`))))

(event `DrawerAnimate`
  ;[0.4055 1 0.5729] Opening Drawer
  (`KismetSystemLibrary.PrintString` "anima")
  (bind (_direction _drawer) (`Timeline|Drawer` :!via `PlayFromStart`)
    (:`Update`
      (`SceneComponent.K2_SetRelativeLocation` (`self.Mesh_Nightstand_Drawer`) (`KismetMathLibrary.VLerp` (`self.StartLocation`) (`self.EndLocation`) _drawer) false false))
    (:`Finished`
      (set `self.?Wait` false))))

(event `AnimateDoor`
  ;[0.4055 1 0.5729] Opening Door Left
  (bind (_direction _drawer) (`Timeline|Door` :!via `PlayFromStart`)
    (:`Update`
      (`SceneComponent.K2_SetRelativeRotation` (`self.Mesh_Nightstand_Door`) (`KismetMathLibrary.RLerp` (`self.StartRotation`) (`self.EndRottation`) _drawer) false false))
    (:`Finished`
      (set `self.?Wait` false))))

(fn `InteractDoor`
  (bind (_relativerotation_roll _relativerotation_pitch _relativerotation_yaw) (`KismetMathLibrary.BreakRotator` (`SceneComponent.RelativeRotation` (`self.Mesh_Nightstand_Door`))))
  (bind (_relativerotation_roll_2 _relativerotation_pitch_2 _relativerotation_yaw_2) (`KismetMathLibrary.BreakRotator` (`SceneComponent.RelativeRotation` (`self.Mesh_Nightstand_Door`))))
  (bind (_relativerotation_roll_3 _relativerotation_pitch_3 _relativerotation_yaw_3) (`KismetMathLibrary.BreakRotator` (`SceneComponent.RelativeRotation` (`self.Mesh_Nightstand_Door`))))
  (if (not (>= _relativerotation_yaw_2 109.0))
    (set `self.StartRotation` (`KismetMathLibrary.MakeRotator` _relativerotation_roll_3 _relativerotation_pitch_3 _relativerotation_yaw_3))
    (set `self.EndRottation` (`KismetMathLibrary.MakeRotator` _relativerotation_roll_3 _relativerotation_pitch_3 110.0))
    (`self.AnimateDoor`)
    (else
      (set `self.StartRotation` (`KismetMathLibrary.MakeRotator` _relativerotation_roll _relativerotation_pitch _relativerotation_yaw))
      (set `self.EndRottation` (`KismetMathLibrary.MakeRotator` _relativerotation_roll _relativerotation_pitch))
      (`self.AnimateDoor`))))

(fn `InteractDrawer`
  (bind (_relativelocation_x _relativelocation_y) (`KismetMathLibrary.BreakVector` (`SceneComponent.RelativeLocation` (`self.Mesh_Nightstand_Drawer`))))
  (bind (_relativelocation_x_2 _relativelocation_y_2 _relativelocation_z) (`KismetMathLibrary.BreakVector` (`SceneComponent.RelativeLocation` (`self.Mesh_Nightstand_Drawer`))))
  (bind (_relativelocation_x_3 _relativelocation_y_3 _relativelocation_z_2) (`KismetMathLibrary.BreakVector` (`SceneComponent.RelativeLocation` (`self.Mesh_Nightstand_Drawer`))))
  (if (not (>= _relativelocation_y 47.0))
    (`KismetSystemLibrary.PrintString` "Playe open sound")
    (set `self.StartLocation` (`KismetMathLibrary.MakeVector` _relativelocation_x_3 _relativelocation_y_3 _relativelocation_z_2))
    (set `self.EndLocation` (`KismetMathLibrary.MakeVector` _relativelocation_x_3 (`self.EndDrawer`) _relativelocation_z_2))
    (`self.DrawerAnimate`)
    (else
      (`KismetSystemLibrary.PrintString` "play close sound")
      (set `self.StartLocation` (`KismetMathLibrary.MakeVector` _relativelocation_x_2 _relativelocation_y_2 _relativelocation_z))
      (set `self.EndLocation` (`KismetMathLibrary.MakeVector` _relativelocation_x_2 (`self.StartDrawer`) _relativelocation_z))
      (`self.DrawerAnimate`))))

(fn `InteractMesh`
  (params (`Outline?` :type Boolean))
  (set `self.Outline?` `Outline?`)
  (if (not (== (`self.Mesh_Nightstand`) (`self.CurrentMesh`)))
    (`PrimitiveComponent.SetRenderCustomDepth` (`self.CurrentMesh`) (`self.Outline?`))
    (if (== (`self.CurrentMesh`) (`self.Mesh_Nightstand_Door`))
      (`SceneComponent.SetVisibility` (`self.DoorRight`) (`self.Outline?`) false)
      (elif (== (`self.CurrentMesh`) (`self.Mesh_Nightstand_Drawer`))
        (`SceneComponent.SetVisibility` (`self.DrawerLeft`) (`self.Outline?`) false)))))

(fn `Open/Close Stuff`
  (if (`self.?Wait`)
    _
    (elif (== (`self.CurrentMesh`) (`self.Mesh_Nightstand_Door`))
      (set `self.?Wait` true)
      (`self.InteractDoor`)
      (elif (== (`self.CurrentMesh`) (`self.Mesh_Nightstand_Drawer`))
        (set `self.?Wait` true)
        (`self.InteractDrawer`)
        (else
          (`KismetSystemLibrary.PrintString` "mepep"))))))

(fn `UserConstructionScript`)