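; Interactable decorative box whose lid the player can open and close.
; While the player is inside the BorderBox overlap, look-at events highlight the targeted mesh, excluding the box body, with a custom-depth outline and show a widget.
; Interacting picks the target roll from the lid's current rotation, then a timeline lerps it open or closed, with a Wait flag blocking input until it finishes.
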(event `/Game/ThirdPerson/Blueprints/BI_InteractableObjects.LookAtObjectMesh`
  (params (HitComponent :type "ActorComponent Object Reference") (`?LookAt` :type Boolean))
  ;[1 0.1086 0.7114] Mesh checking  -> outline already there
  (bind _output_get (set `self.? Look At` `?LookAt`))
  (if (`self.?Wait`)
    _
    (elif (`self.?NearObject`)
      (if _output_get
        (bind _asstatic_mesh_component (cast `StaticMeshComponent` HitComponent))
        (set `self.LookAtMesh` _asstatic_mesh_component)
        (if (== (`self.CurrentMesh`) (`self.LookAtMesh`))
          (`self.InteractMesh` true)
          (else
            (`/Engine/EditorBlueprintResources/StandardMacros.IsValid` (`self.CurrentMesh`)
              (:`Is Valid`
                (`PrimitiveComponent.SetRenderCustomDepth` (`self.decoration_box_cap`) false)
                (`SceneComponent.SetVisibility` (`self.Widget`) false false)
                (set `self.CurrentMesh` (`self.LookAtMesh`))
                (`self.InteractMesh` true))
              (:`Is Not Valid`
                (set `self.CurrentMesh` (`self.LookAtMesh`))
                (`self.InteractMesh` true)))))
        (else
          (`PrimitiveComponent.SetRenderCustomDepth` (`self.decoration_box_cap`) false)
          (`SceneComponent.SetVisibility` (`self.Widget`) false false))))))

(event `/Game/ThirdPerson/Blueprints/BI_InteractableObjects.InteractWith`
  ;[1 1 1] Comment
  (if (not (== (`self.decoration_box`) (`self.CurrentMesh`)))
    (if (`self.? Look At`)
      (if (not (`self.?Wait`))
        (`self.Open/Close Stuff`)))))

(event `self.BorderBox.OnComponentBeginOverlap`
  (params (OverlappedComponent :type "PrimitiveComponent Object Reference") (OtherActor :type "Actor Object Reference") (OtherComp :type "PrimitiveComponent Object Reference") (OtherBodyIndex :type Integer) (bFromSweep :type Boolean) (SweepResult :type "HitResult Structure (by ref)"))
  (set `self.?NearObject` true))

(event `AnimateLid`
  ;[0.4055 1 0.5729] Opening Lid
  (bind (_direction _drawer) (`Timeline|Timeline` :!via `PlayFromStart`)
    (:`Update`
      (`SceneComponent.K2_SetRelativeRotation` (`self.decoration_box_cap`) (`KismetMathLibrary.RLerp` (`self.StartRotation`) (`self.EndRottation`) _drawer) false false))
    (:`Finished`
      (set `self.?Wait` false))))

(event `self.BorderBox.OnComponentEndOverlap`
  (params (OverlappedComponent :type "PrimitiveComponent Object Reference") (OtherActor :type "Actor Object Reference") (OtherComp :type "PrimitiveComponent Object Reference") (OtherBodyIndex :type Integer))
  (set `self.?NearObject` false)
  (`PrimitiveComponent.SetRenderCustomDepth` (`self.decoration_box_cap`) false)
  (`SceneComponent.SetVisibility` (`self.Widget`) false false))

(fn `InteractMesh`
  (params (`Outline?` :type Boolean))
  (set `self.Outline?` `Outline?`)
  (if (not (== (`self.decoration_box`) (`self.CurrentMesh`)))
    (`PrimitiveComponent.SetRenderCustomDepth` (`self.CurrentMesh`) (`local.Outline?`))
    (`SceneComponent.SetVisibility` (`self.Widget`) true false)))

(fn `Open/Close Stuff`
  (if (not (`self.?Wait`))
    (set `self.?Wait` true)
    (`self.OpenLid`)))

(fn `OpenLid`
  (bind (_relativerotation_roll _relativerotation_pitch _relativerotation_yaw) (`KismetMathLibrary.BreakRotator` (`SceneComponent.RelativeRotation` (`self.decoration_box_cap`))))
  (bind _relativerotation_roll_2 (`KismetMathLibrary.BreakRotator` (`SceneComponent.RelativeRotation` (`self.decoration_box_cap`))))
  (bind (_relativerotation_roll_3 _relativerotation_pitch_2 _relativerotation_yaw_2) (`KismetMathLibrary.BreakRotator` (`SceneComponent.RelativeRotation` (`self.decoration_box_cap`))))
  (if (not (<= _relativerotation_roll_2 -35.0))
    (set `self.StartRotation` (`KismetMathLibrary.MakeRotator` _relativerotation_roll_3 _relativerotation_pitch_2 _relativerotation_yaw_2))
    (set `self.EndRottation` (`KismetMathLibrary.MakeRotator` -45.0 _relativerotation_pitch_2 _relativerotation_yaw_2))
    (else
      (set `self.StartRotation` (`KismetMathLibrary.MakeRotator` _relativerotation_roll _relativerotation_pitch _relativerotation_yaw))
      (set `self.EndRottation` (`KismetMathLibrary.MakeRotator` 0.0 _relativerotation_pitch _relativerotation_yaw))))
  (`self.AnimateLid`))

(fn `UserConstructionScript`)