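; Medicine storage cabinet actor with many small, medium and large drawers that slide open and closed on interaction.
; Look-at events outline the hovered drawer via custom depth and show its widget, using parallel mesh and widget arrays to match and clear highlights.
; Interacting picks open or closed from the drawer's X position, then a timeline lerps it along X while a Wait flag blocks input until finished.
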(event `self.ReceiveBeginPlay`
  ;[0.08854 0.08854 0.08854] arrays for easy outline removale
  (set `self.Mesh Array` (`|MakeArray` (`self.DrawerSmall12`) (`self.DrawerSmall9`) (`self.DrawerSmall7`) (`self.DrawerSmall4`) (`self.DrawerSmall3`) (`self.DrawerSmall2`) (`self.DrawerSmall1`) (`self.DrawerSmall8`) (`self.DrawerSmall16`) (`self.DrawerSmall17`) (`self.DrawerSmall18`) (`self.DrawerSmall14`) (`self.DrawerSmall10`) (`self.DrawerSmall11`) (`self.DrawerSmall15`) (`self.DrawerSmall13`) (`self.DrawerMedium2`) (`self.DrawerMedium1`) (`self.DrawerMedium3`) (`self.DrawerLarge3`) (`self.DrawerLarge2`) (`self.DrawerLarge1`) (`self.DrawerMedium4`) (`self.DrawerMedium8`) (`self.DrawerSmall5`) (`self.DrawerMedium11`) (`self.DrawerMedium12`) (`self.DrawerSmall6`) (`self.DrawerMedium9`) (`self.DrawerMedium6`) (`self.DrawerMedium5`) (`self.DrawerMedium7`) (`self.DrawerMedium10`)))
  (set `self.Widget Array` (`|MakeArray` (`self.WidgetDrawerS12`) (`self.WidgetDrawerS9`) (`self.WidgetDrawerS7`) (`self.WidgetDrawerS4`) (`self.WidgetDrawerS3`) (`self.WidgetDrawerS2`) (`self.WidgetDrawerS1`) (`self.WidgetDrawerS8`) (`self.WidgetDrawerS16`) (`self.WidgetDrawerS17`) (`self.WidgetDrawerS18`) (`self.WidgetDrawerS14`) (`self.WidgetDrawerS10`) (`self.WidgetDrawerS11`) (`self.WidgetDrawerS15`) (`self.WidgetDrawerS13`) (`self.WidgetDrawerM2`) (`self.WidgetDrawerM1`) (`self.WidgetDrawerM3`) (`self.WidgetDrawerL3`) (`self.WidgetDrawerL2`) (`self.WidgetDrawerL1`) (`self.WidgetDrawerM4`) (`self.WidgetDrawerM8`) (`self.WidgetDrawerS5`) (`self.WidgetDrawerM11`) (`self.WidgetDrawerM12`) (`self.WidgetDrawerS6`) (`self.WidgetDrawerM9`) (`self.WidgetDrawerM6`) (`self.WidgetDrawerM5`) (`self.WidgetDrawerM7`) (`self.WidgetDrawerM10`))))

(event `/Game/ThirdPerson/Blueprints/BI_InteractableObjects.LookAtObjectMesh`
  (params (HitComponent :type "ActorComponent Object Reference") (`?LookAt` :type Boolean))
  ;[1 0.1086 0.7114] Mesh checking  -> outline already there
  (if (not (`self.?Wait`))
    (bind _output_get (set `self.? Look At` `?LookAt`))
    (if _output_get
      (bind _asstatic_mesh_component (cast `StaticMeshComponent` HitComponent))
      (set `self.LookAtMesh` _asstatic_mesh_component)
      (if (== (`self.CurrentMesh`) (`self.LookAtMesh`))
        (`self.InteractMesh` true)
        (else
          (`/Engine/EditorBlueprintResources/StandardMacros.IsValid` (`self.CurrentMesh`)
            (:`Is Valid`
              (for _array_element (`self.Mesh Array`)
                (`PrimitiveComponent.SetRenderCustomDepth` _array_element false))
              (for _array_element_2 (`self.Widget Array`)
                (`SceneComponent.SetVisibility` _array_element_2 false false))
              (set `self.CurrentMesh` (`self.LookAtMesh`))
              (`self.InteractMesh` true))
            (:`Is Not Valid`
              (set `self.CurrentMesh` (`self.LookAtMesh`))
              (`self.InteractMesh` true)))))
      (else
        (for _array_element_3 (`self.Mesh Array`)
          (`PrimitiveComponent.SetRenderCustomDepth` _array_element_3 false))
        (for _array_element_4 (`self.Widget Array`)
          (`SceneComponent.SetVisibility` _array_element_4 false false))))))

(event `/Game/ThirdPerson/Blueprints/BI_InteractableObjects.InteractWith`
  ;[1 1 1] Comment
  (if (not (== (`self.00case`) (`self.CurrentMesh`)))
    (if (`self.? Look At`)
      (if (not (`self.?Wait`))
        (`self.Open/Close Stuff`)))))

(event `DrawerAnimate`
  ;[0.4055 1 0.5729] Opening Drawer Right
  (bind (_direction _drawer) (`Timeline|Timeline` :!via `PlayFromStart`)
    (:`Update`
      (`SceneComponent.K2_SetRelativeLocation` (`self.CurrentMesh`) (`KismetMathLibrary.VLerp` (`self.StartLocation`) (`self.EndLocation`) _drawer) false false))
    (:`Finished`
      (set `self.?Wait` false))))

(fn `Interact Drawer`
  (bind _relativelocation_x (`KismetMathLibrary.BreakVector` (`SceneComponent.RelativeLocation` (`self.CurrentMesh`))))
  (bind (_relativelocation_x_2 _relativelocation_y _relativelocation_z) (`KismetMathLibrary.BreakVector` (`SceneComponent.RelativeLocation` (`self.CurrentMesh`))))
  (bind (_relativelocation_x_3 _relativelocation_y_2 _relativelocation_z_2) (`KismetMathLibrary.BreakVector` (`SceneComponent.RelativeLocation` (`self.CurrentMesh`))))
  (if (not (>= _relativelocation_x 89.0))
    (set `self.StartLocation` (`KismetMathLibrary.MakeVector` _relativelocation_x_3 _relativelocation_y_2 _relativelocation_z_2))
    (set `self.EndLocation` (`KismetMathLibrary.MakeVector` (`self.EndDrawer`) _relativelocation_y_2 _relativelocation_z_2))
    (else
      (set `self.StartLocation` (`KismetMathLibrary.MakeVector` _relativelocation_x_2 _relativelocation_y _relativelocation_z))
      (set `self.EndLocation` (`KismetMathLibrary.MakeVector` 0.0 _relativelocation_y _relativelocation_z))))
  (`self.DrawerAnimate`))

(fn `InteractMesh`
  (params (`Outline?` :type Boolean))
  (set `self.Outline?` `Outline?`)
  (if (not (== (`self.00case`) (`self.CurrentMesh`)))
    (`PrimitiveComponent.SetRenderCustomDepth` (`self.CurrentMesh`) (`local.Outline?`))
    (`SceneComponent.SetVisibility` (`|GetArrayItem` (`self.Widget Array`) (`KismetArrayLibrary.Array_Find` (`self.Mesh Array`) (`self.CurrentMesh`))) true false)))

(fn `Open/Close Stuff`
  (if (not (`self.?Wait`))
    (set `self.?Wait` true)
    (`self.Interact Drawer`)))

(fn `UserConstructionScript`)