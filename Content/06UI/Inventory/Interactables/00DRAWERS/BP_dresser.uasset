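; Interactable dresser with three drawers and two doors that the player highlights by looking at them and opens or closes on interact.
; LookatObjectMesh tracks the hit component, toggling its custom-depth outline and matching widget, and clearing the others via mesh and widget arrays.
; Interactwith picks the open or closed target from the part's current transform, then a Timeline lerps it there while a shared Wait flag blocks further interaction.
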(event `self.ReceiveBeginPlay`
  ;[0.08854 0.08854 0.08854] arrays for easy outline removale
  (set `self.Mesh Array` (`|MakeArray` (`self.dresser_drawer`) (`self.dresser_drawer2`) (`self.dresser_drawer3`) (`self.dresser_leftdoor`) (`self.dresser_rightdoor`)))
  (set `self.Widget Array` (`|MakeArray` (`self.Drawer3`) (`self.Drawer2`) (`self.Drawer`) (`self.DoorLeft`) (`self.DoorRight`))))

(event `/Game/ThirdPerson/Blueprints/BI_InteractableObjects.LookAtObjectMesh`
  (params (HitComponent :type "ActorComponent Object Reference") (`?LookAt` :type Boolean))
  ;[1 0.1086 0.7114] Mesh checking  -> outline already there
  (bind _output_get (set `self.? Look At` `?LookAt`))
  (if _output_get
    (bind _asstatic_mesh_component (cast `StaticMeshComponent` HitComponent)
      (:`then`
        (set `self.LookAtMesh` _asstatic_mesh_component)
        (if (== (`self.CurrentMesh`) (`self.LookAtMesh`))
          (`self.InteractMesh` true)
          (else
            (`/Engine/EditorBlueprintResources/StandardMacros.IsValid` (`self.CurrentMesh`)
              (:`Is Valid`
                (for _array_element (`self.Mesh Array`)
                  (`PrimitiveComponent.SetRenderCustomDepth` _array_element false))
                (for _array_element_2 (`self.Widget Array`)
                  (`SceneComponent.SetVisibility` _array_element_2 false false))
                (set `self.CurrentMesh` (`self.LookAtMesh`))
                (`self.InteractMesh` true))
              (:`Is Not Valid`
                (set `self.CurrentMesh` (`self.LookAtMesh`))
                (`self.InteractMesh` true))))))
      (:`CastFailed`
        (`KismetSystemLibrary.PrintString` "cast faild object")))
    (else
      (for _array_element_3 (`self.Mesh Array`)
        (`PrimitiveComponent.SetRenderCustomDepth` _array_element_3 false))
      (for _array_element_4 (`self.Widget Array`)
        (`SceneComponent.SetVisibility` _array_element_4 false false)))))

(event `/Game/ThirdPerson/Blueprints/BI_InteractableObjects.InteractWith`
  ;[1 1 1] Comment
  (if (`self.? Look At`)
    (if (not (`self.?Wait`))
      (`self.Open/Close Stuff`))))

(event `DrawerAnimate`
  ;[0.4055 1 0.5729] Opening Drawer Right
  (`KismetSystemLibrary.PrintString` "anima")
  (bind (_direction _drawer) (`Timeline|Timeline` :!via `PlayFromStart`)
    (:`Update`
      (`SceneComponent.K2_SetRelativeLocation` (`self.dresser_drawer`) (`KismetMathLibrary.VLerp` (`self.StartLocation`) (`self.EndLocation`) _drawer) false false))
    (:`Finished`
      (set `self.?Wait` false))))

(event `AnimateDrawer3`
  ;[0.4055 1 0.5729] Opening Drawer Left
  (bind (_direction _drawer) (`Timeline|Timeline_3` :!via `PlayFromStart`)
    (:`Update`
      (`SceneComponent.K2_SetRelativeLocation` (`self.dresser_drawer3`) (`KismetMathLibrary.VLerp` (`self.StartLocation`) (`self.EndLocation`) _drawer) false false))
    (:`Finished`
      (set `self.?Wait` false))))

(event `DrawerAnimate2`
  ;[0.4055 1 0.5729] Opening Drawer Left
  (bind (_direction _drawer) (`Timeline|Timeline_0` :!via `PlayFromStart`)
    (:`Update`
      (`SceneComponent.K2_SetRelativeLocation` (`self.dresser_drawer2`) (`KismetMathLibrary.VLerp` (`self.StartLocation`) (`self.EndLocation`) _drawer) false false))
    (:`Finished`
      (set `self.?Wait` false))))

(event `AnimateDoorRight`
  ;[0.4055 1 0.5729] Opening Door Right
  (bind (_direction _drawer) (`Timeline|Timeline_1` :!via `PlayFromStart`)
    (:`Update`
      (`SceneComponent.K2_SetRelativeRotation` (`self.dresser_rightdoor`) (`KismetMathLibrary.RLerp` (`self.StartRotation`) (`self.EndRottation`) _drawer) false false))
    (:`Finished`
      (set `self.?Wait` false))))

(event `AnimateDoorLeft`
  ;[0.4055 1 0.5729] Opening Door Left
  (bind (_direction _drawer) (`Timeline|Timeline_2` :!via `PlayFromStart`)
    (:`Update`
      (`SceneComponent.K2_SetRelativeRotation` (`self.dresser_leftdoor`) (`KismetMathLibrary.RLerp` (`self.StartRotation`) (`self.EndRottation`) _drawer) false false))
    (:`Finished`
      (set `self.?Wait` false))))

(fn `InteractDoorLeft`
  (bind (_relativerotation_roll _relativerotation_pitch _relativerotation_yaw) (`KismetMathLibrary.BreakRotator` (`SceneComponent.RelativeRotation` (`self.dresser_leftdoor`))))
  (bind (_relativerotation_roll_2 _relativerotation_pitch_2 _relativerotation_yaw_2) (`KismetMathLibrary.BreakRotator` (`SceneComponent.RelativeRotation` (`self.dresser_leftdoor`))))
  (bind (_relativerotation_roll_3 _relativerotation_pitch_3 _relativerotation_yaw_3) (`KismetMathLibrary.BreakRotator` (`SceneComponent.RelativeRotation` (`self.dresser_leftdoor`))))
  (if (not (>= _relativerotation_yaw_2 109.0))
    (set `self.StartRotation` (`KismetMathLibrary.MakeRotator` _relativerotation_roll_3 _relativerotation_pitch_3 _relativerotation_yaw_3))
    (set `self.EndRottation` (`KismetMathLibrary.MakeRotator` _relativerotation_roll_3 _relativerotation_pitch_3 110.0))
    (`self.AnimateDoorLeft`)
    (else
      (set `self.StartRotation` (`KismetMathLibrary.MakeRotator` _relativerotation_roll _relativerotation_pitch _relativerotation_yaw))
      (set `self.EndRottation` (`KismetMathLibrary.MakeRotator` _relativerotation_roll _relativerotation_pitch))
      (`self.AnimateDoorLeft`))))

(fn `InteractDoorRight`
  (bind (_relativerotation_roll _relativerotation_pitch _relativerotation_yaw) (`KismetMathLibrary.BreakRotator` (`SceneComponent.RelativeRotation` (`self.dresser_rightdoor`))))
  (bind (_relativerotation_roll_2 _relativerotation_pitch_2 _relativerotation_yaw_2) (`KismetMathLibrary.BreakRotator` (`SceneComponent.RelativeRotation` (`self.dresser_rightdoor`))))
  (bind (_relativerotation_roll_3 _relativerotation_pitch_3 _relativerotation_yaw_3) (`KismetMathLibrary.BreakRotator` (`SceneComponent.RelativeRotation` (`self.dresser_rightdoor`))))
  (if (not (<= _relativerotation_yaw_2 -109.0))
    (set `self.StartRotation` (`KismetMathLibrary.MakeRotator` _relativerotation_roll_3 _relativerotation_pitch_3 _relativerotation_yaw_3))
    (set `self.EndRottation` (`KismetMathLibrary.MakeRotator` _relativerotation_roll_3 _relativerotation_pitch_3 -110.0))
    (`self.AnimateDoorRight`)
    (else
      (set `self.StartRotation` (`KismetMathLibrary.MakeRotator` _relativerotation_roll _relativerotation_pitch _relativerotation_yaw))
      (set `self.EndRottation` (`KismetMathLibrary.MakeRotator` _relativerotation_roll _relativerotation_pitch))
      (`self.AnimateDoorRight`))))

(fn `InteractDrawerLeft`
  (bind (_relativelocation_x _relativelocation_y) (`KismetMathLibrary.BreakVector` (`SceneComponent.RelativeLocation` (`self.dresser_drawer2`))))
  (bind (_relativelocation_x_2 _relativelocation_y_2 _relativelocation_z) (`KismetMathLibrary.BreakVector` (`SceneComponent.RelativeLocation` (`self.dresser_drawer2`))))
  (bind (_relativelocation_x_3 _relativelocation_y_3 _relativelocation_z_2) (`KismetMathLibrary.BreakVector` (`SceneComponent.RelativeLocation` (`self.dresser_drawer2`))))
  (if (not (>= _relativelocation_y 35.0))
    (set `self.StartLocation` (`KismetMathLibrary.MakeVector` _relativelocation_x_3 _relativelocation_y_3 _relativelocation_z_2))
    (set `self.EndLocation` (`KismetMathLibrary.MakeVector` _relativelocation_x_3 (`self.EndDrawer`) _relativelocation_z_2))
    (else
      (set `self.StartLocation` (`KismetMathLibrary.MakeVector` _relativelocation_x_2 _relativelocation_y_2 _relativelocation_z))
      (set `self.EndLocation` (`KismetMathLibrary.MakeVector` _relativelocation_x_2 (`self.StartDrawer`) _relativelocation_z))))
  (`self.DrawerAnimate2`) ; Opening
)

(fn `InteractDrawerMiddle`
  (bind (_relativelocation_x _relativelocation_y) (`KismetMathLibrary.BreakVector` (`SceneComponent.RelativeLocation` (`self.dresser_drawer3`))))
  (bind (_relativelocation_x_2 _relativelocation_y_2 _relativelocation_z) (`KismetMathLibrary.BreakVector` (`SceneComponent.RelativeLocation` (`self.dresser_drawer3`))))
  (bind (_relativelocation_x_3 _relativelocation_y_3 _relativelocation_z_2) (`KismetMathLibrary.BreakVector` (`SceneComponent.RelativeLocation` (`self.dresser_drawer3`))))
  (if (not (>= _relativelocation_y 35.0))
    (set `self.StartLocation` (`KismetMathLibrary.MakeVector` _relativelocation_x_3 _relativelocation_y_3 _relativelocation_z_2))
    (set `self.EndLocation` (`KismetMathLibrary.MakeVector` _relativelocation_x_3 (`self.EndDrawer`) _relativelocation_z_2))
    (else
      (set `self.StartLocation` (`KismetMathLibrary.MakeVector` _relativelocation_x_2 _relativelocation_y_2 _relativelocation_z))
      (set `self.EndLocation` (`KismetMathLibrary.MakeVector` _relativelocation_x_2 (`self.StartDrawer`) _relativelocation_z))))
  (`self.AnimateDrawer3`))

(fn `InteractDrawerRight`
  (bind (_relativelocation_x _relativelocation_y) (`KismetMathLibrary.BreakVector` (`SceneComponent.RelativeLocation` (`self.dresser_drawer`))))
  (bind (_relativelocation_x_2 _relativelocation_y_2 _relativelocation_z) (`KismetMathLibrary.BreakVector` (`SceneComponent.RelativeLocation` (`self.dresser_drawer`))))
  (bind (_relativelocation_x_3 _relativelocation_y_3 _relativelocation_z_2) (`KismetMathLibrary.BreakVector` (`SceneComponent.RelativeLocation` (`self.dresser_drawer`))))
  (if (not (>= _relativelocation_y 35.0))
    (`KismetSystemLibrary.PrintString` "Playe open sound")
    (set `self.StartLocation` (`KismetMathLibrary.MakeVector` _relativelocation_x_3 _relativelocation_y_3 _relativelocation_z_2))
    (set `self.EndLocation` (`KismetMathLibrary.MakeVector` _relativelocation_x_3 (`self.EndDrawer`) _relativelocation_z_2))
    (`self.DrawerAnimate`)
    (else
      (`KismetSystemLibrary.PrintString` "play close sound")
      (set `self.StartLocation` (`KismetMathLibrary.MakeVector` _relativelocation_x_2 _relativelocation_y_2 _relativelocation_z))
      (set `self.EndLocation` (`KismetMathLibrary.MakeVector` _relativelocation_x_2 (`self.StartDrawer`) _relativelocation_z))
      (`self.DrawerAnimate`))))

(fn `InteractMesh`
  (params (`Outline?` :type Boolean))
  (set `self.Outline?` `Outline?`)
  (if (not (== (`self.dresser`) (`self.CurrentMesh`)))
    (`PrimitiveComponent.SetRenderCustomDepth` (`self.CurrentMesh`) (`self.Outline?`))
    (if (== (`self.CurrentMesh`) (`self.dresser_drawer`))
      (`SceneComponent.SetVisibility` (`self.Drawer`) (`self.Outline?`) false)
      (elif (== (`self.CurrentMesh`) (`self.dresser_drawer2`))
        (`SceneComponent.SetVisibility` (`self.Drawer2`) (`self.Outline?`) false)
        (elif (== (`self.CurrentMesh`) (`self.dresser_drawer3`))
          (`SceneComponent.SetVisibility` (`self.Drawer3`) (`self.Outline?`) false)
          (elif (== (`self.CurrentMesh`) (`self.dresser_leftdoor`))
            (`SceneComponent.SetVisibility` (`self.DoorLeft`) (`self.Outline?`) false)
            (elif (== (`self.CurrentMesh`) (`self.dresser_rightdoor`))
              (`SceneComponent.SetVisibility` (`self.DoorRight`) (`self.Outline?`) false))))))))

(fn `Open/Close Stuff`
  (if (`self.?Wait`)
    _
    (elif (== (`self.CurrentMesh`) (`self.dresser_rightdoor`))
      (set `self.?Wait` true)
      (`self.InteractDoorRight`)
      (elif (== (`self.CurrentMesh`) (`self.dresser_leftdoor`))
        (set `self.?Wait` true)
        (`self.InteractDoorLeft`)
        (elif (== (`self.CurrentMesh`) (`self.dresser_drawer`))
          (set `self.?Wait` true)
          (`self.InteractDrawerRight`)
          (elif (== (`self.CurrentMesh`) (`self.dresser_drawer2`))
            (set `self.?Wait` true)
            (`self.InteractDrawerLeft`)
            (elif (== (`self.CurrentMesh`) (`self.dresser_drawer3`))
              (set `self.?Wait` true)
              (`self.InteractDrawerMiddle`))))))))

(fn `UserConstructionScript`)