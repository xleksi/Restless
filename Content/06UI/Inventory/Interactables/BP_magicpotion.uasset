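; BP_magicpotion is an interactable magic potion pickup placed in the world.
; When looked at, it toggles custom depth rendering on its mesh and shows or hides its widget.
; On pickup, it calls ActivateMagic on every top-level WBP_HUDonScreen widget, then destroys itself.
; Both events still print debug strings.
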(event `/Game/06UI/Inventory/Interactables/BI_MagicPotion.SetLookAt`
  (params (`?LookingAt` :type Boolean))
  (`PrimitiveComponent.SetRenderCustomDepth` (`self.Magicpotion`) `?LookingAt`)
  (`SceneComponent.SetVisibility` (`self.Widget`) `?LookingAt` false)
  (`KismetSystemLibrary.PrintString` "Hello"))

(event `/Game/06UI/Inventory/Interactables/BI_MagicPotion.Pickup`
  (`KismetSystemLibrary.PrintString` "e")
  (bind _foundwidgets (`WidgetBlueprintLibrary.GetAllWidgetsOfClass` "/Game/06UI/HUDonScreen/WBP_HUDonScreen.WBP_HUDonScreen_C"))
  (for _array_element _foundwidgets
    (`/Game/06UI/HUDonScreen/WBP_MagicAbility.ActivateMagic` _array_element))
  (`self.K2_DestroyActor`))

(fn `UserConstructionScript`)