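; BP_Door1 is an interactable locked door that opens once when the player holds a key.
; Box overlap shows the interact widget and tracks player overlap, while GetKey and KeyUsed maintain key items and count.
; Interact plays an unlock sound and rotates the mesh via a timeline, then consumes a key from its owning inventory; without keys, message-box widgets show a no-key message.
; Direction-based swing logic is present but unused.
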(event `/Game/06UI/Inventory/Interfaces/BI_InteractDoor.Interact`
  (params (PlayerLocation :type "Vector Structure"))
  (bind _output (`|GetArrayItem` (`self.KeyInfo`) (`self.Counter`)))
  ;[1 1 1] Opening Door
  (if (> (`self.AvaiableKeys`) 0)
    (`/Engine/EditorBlueprintResources/StandardMacros.DoOnce` false
      (:`Completed`
        ;;[1 0.8392 0.01883] sfx_unlock the door
        (`GameplayStatics.PlaySound2D` "/Game/06UI/Inventory/Interactables/Door/louder_unlock_the_door_ncc0.louder_unlock_the_door_ncc0" 1.0 1.0 0.0 null null)
        (bind (_direction _open) (`Timeline|Open`)
          (:`Update`
            (`SceneComponent.K2_SetRelativeRotation` (`self.SketchFab_FBX_All_Modules_door`) (`KismetMathLibrary.MakeRotator` 0.0 0.0 _open) false false))
          (:`Finished`
            (`/Game/06UI/Inventory/AC_InventoryComponent.ConsumeItem` (`.OwningInventory_7_A777FCB449167D1A2B913EB63BD67415` (break `/Game/06UI/Inventory/F_InventoryItem` _output)) _output)
            (`/Engine/EditorBlueprintResources/StandardMacros.IncrementInt` (`self.Counter`))))))
    (else
      (bind _foundwidgets (`WidgetBlueprintLibrary.GetAllWidgetsWithInterface` "/Game/06UI/Inventory/Interfaces/BI_MessageBox.BI_MessageBox_C"))
      (message `/Game/06UI/Inventory/Interfaces/BI_MessageBox.NoKeyMessage` _foundwidgets))))

(event `self.Box.OnComponentBeginOverlap`
  (params (OverlappedComponent :type "PrimitiveComponent Object Reference") (OtherActor :type "Actor Object Reference") (OtherComp :type "PrimitiveComponent Object Reference") (OtherBodyIndex :type Integer) (bFromSweep :type Boolean) (SweepResult :type "HitResult Structure (by ref)"))
  ;[1 1 1] Overlapping with Player, Shows Interact Text
  (`SceneComponent.SetVisibility` (`self.Widget`) true false)
  ;;[0.1817 0.349 0.2162] Set bIsOverlapping true/false
  (if (== OtherActor (`GameplayStatics.GetPlayerCharacter` 0))
    (set `self.bIsOverlapping` true)))

(event `self.Box.OnComponentEndOverlap`
  (params (OverlappedComponent :type "PrimitiveComponent Object Reference") (OtherActor :type "Actor Object Reference") (OtherComp :type "PrimitiveComponent Object Reference") (OtherBodyIndex :type Integer))
  ;[1 1 1] Overlapping with Player, Shows Interact Text
  (`SceneComponent.SetVisibility` (`self.Widget`) false false)
  ;;[0.1817 0.349 0.2162] Set bIsOverlapping true/false
  (if (== (`GameplayStatics.GetPlayerCharacter` 0) OtherActor)
    (set `self.bIsOverlapping` false)))

(event `/Game/06UI/Inventory/Interfaces/BI_InteractDoor.getKey`
  (params (Item :type "/Game/06UI/Inventory/F_InventoryItem Structure"))
  ;[1 1 1] Getting Info When Player gets a key
  (set `self.Item` Item)
  (`KismetArrayLibrary.Array_Add` (`self.KeyInfo`) (`self.Item`))
  (`/Engine/EditorBlueprintResources/StandardMacros.IncrementInt` (`self.AvaiableKeys`)))

(event `/Game/06UI/Inventory/Interfaces/BI_InteractDoor.KeyUsed`
  (params (Item :type "/Game/06UI/Inventory/F_InventoryItem Structure"))
  ;[1 1 1] Make the Avaiable Key-Count lower
  (`/Engine/EditorBlueprintResources/StandardMacros.DecrementInt` (`self.AvaiableKeys`)))

(fn `GetItemData`
  (returns (ItemClass :type "Actor Class Reference") (CurrentStackSize :type Integer) (MaxStackSize :type Integer))
  (return null 0 0))

(fn `OverlapWithPlayer`
  (returns (`?Overlapping` :type Boolean))
  (return (`self.bIsOverlapping`)))

(fn `UpdateKeyParts`
  (returns (NewParam :type Integer) (NewParam1 :type Integer))
  (return 0 0))

(fn `UserConstructionScript`)