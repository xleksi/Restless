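; BP_bed_boss is an interactable bed hiding place for the player.
; Overlapping its trigger shows an interact prompt, stores the character and enables gated Hide input, which toggles hiding.
; Hiding blends the view to the bed, where a Delay-driven self-calling event rotates the under-bed camera from Turn and Lookup input with clamped pitch.
; When the player is not hiding, those axes drive the character's controller.
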(event `InputAction|Hide`
  (params (Key :type "Key Structure"))
  (bind _char_ref (`self.Char REF`))
  (:`Pressed`
    (`/Engine/EditorBlueprintResources/StandardMacros.Gate` true :!label _label
      (:`Exit`
        (if (`/Game/ThirdPerson/Blueprints/BP_ThirdPersonCharacter.IsHiding` _char_ref)
          (`/Game/ThirdPerson/Blueprints/BP_ThirdPersonCharacter.Unhide` _char_ref)
          (else
            (`/Game/ThirdPerson/Blueprints/BP_ThirdPersonCharacter.Hide` _char_ref)
            (`|ExecutionSequence`
              (:`then_0`
                ;[1 1 1] switch camera view into bed
                (`PlayerController.SetViewTargetWithBlend` (`GameplayStatics.GetPlayerController` 0) self 0.5 "VTBlend_Linear" 0.0 false)
                (`self.MoveCamera`))
              (:`then_1`
                (`KismetSystemLibrary.Delay` 0.2)
                (`self.EnableInput` (`GameplayStatics.GetPlayerController` 0) :!label _label_2)
                (goto _label :!via `Open`)))))))))

(event `self.collision_for_hiding.OnComponentBeginOverlap`
  (params (OverlappedComponent :type "PrimitiveComponent Object Reference") (OtherActor :type "Actor Object Reference") (OtherComp :type "PrimitiveComponent Object Reference") (OtherBodyIndex :type Integer) (bFromSweep :type Boolean) (SweepResult :type "HitResult Structure (by ref)"))
  (if (== OtherActor (`GameplayStatics.GetPlayerCharacter` 0))
    (`SceneComponent.SetVisibility` (`Actor.RootComponent` OtherActor) true false)
    (`SceneComponent.SetVisibility` (`self.EtoInteract`) true false)
    (bind _asbp_third_person_character (cast `/Game/ThirdPerson/Blueprints/BP_ThirdPersonCharacter` OtherActor))
    ;[0.9955 1 0.4293] neat
    (set `self.Char REF` _asbp_third_person_character)
    (goto _label_2)))

(event `self.collision_for_hiding.OnComponentEndOverlap`
  (params (OverlappedComponent :type "PrimitiveComponent Object Reference") (OtherActor :type "Actor Object Reference") (OtherComp :type "PrimitiveComponent Object Reference") (OtherBodyIndex :type Integer))
  (if (== OtherActor (`GameplayStatics.GetPlayerCharacter` 0))
    (`SceneComponent.SetVisibility` (`Actor.RootComponent` OtherActor) false false)
    (`SceneComponent.SetVisibility` (`self.EtoInteract`) false false)
    (cast `/Game/ThirdPerson/Blueprints/BP_ThirdPersonCharacter` OtherActor)
    (`self.DisableInput` (`GameplayStatics.GetPlayerController` 0))
    (goto _label :!via `Close`)))

(event `MoveCamera`
  (if (`/Game/ThirdPerson/Blueprints/BP_ThirdPersonCharacter.IsHiding` (`self.Char REF`))
    (`SceneComponent.K2_SetRelativeRotation` (`self.Camera Under Bed`) (`KismetMathLibrary.MakeRotator` 0.0 (`KismetMathLibrary.FClamp` (+ (stale `InputAxis|Lookup` _output_get) -1.0) -20.0 20.0) (stale `InputAxis|Turn` _output_get)) false false)
    (`KismetSystemLibrary.Delay` 0.001)
    (`self.MoveCamera`)))

(event `InputAxis|Lookup`
  (params (AxisValue :type "Float (single-precision)"))
  (bind _char_ref (`self.Char REF`))
  (if (`/Game/ThirdPerson/Blueprints/BP_ThirdPersonCharacter.IsHiding` _char_ref)
    (bind _output_get (set `self.Pitch` (+ (`self.Pitch`) AxisValue)))
    (else
      (`Pawn.AddControllerPitchInput` _char_ref AxisValue))))

(event `InputAxis|Turn`
  (params (AxisValue :type "Float (single-precision)"))
  (bind _char_ref (`self.Char REF`))
  (if (`/Game/ThirdPerson/Blueprints/BP_ThirdPersonCharacter.IsHiding` _char_ref)
    (bind _output_get (set `self.Yaw` (+ (`self.Yaw`) AxisValue)))
    (else
      (`Pawn.AddControllerYawInput` _char_ref AxisValue))))

(fn `UserConstructionScript`)