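; BP_WorldItem is an interactable inventory pickup that takes its mesh, billboard and name from its Item class defaults.
; SetLookAt toggles a custom-depth highlight and prompt widget.
; Interact, gated by PickedUP, triggers InspectPickUp, which attaches the item to the character before the first- or third-person camera and shows a name widget.
; It then passes the quantity to the inventory, keeping any remainder or destroying itself and the widget after a delay.
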(event `self.ReceiveBeginPlay`
  (`StaticMeshComponent.SetStaticMesh` (`self.DisplayMesh`) (defaults `Object` (`self.Item`))))

(event `Destroy item`
  (`KismetSystemLibrary.Delay` 0.7)
  (bind _foundwidgets (`WidgetBlueprintLibrary.GetAllWidgetsOfClass` "/Game/06UI/Inventory/Widgets/Inspect/WBP_InspectPickUP.WBP_InspectPickUP_C"))
  (for _array_element _foundwidgets
    (`Widget.RemoveFromParent` _array_element)
    (`self.K2_DestroyActor`)))

(fn `GetInspectDistance`
  (returns (NewParam :type "Float (double-precision)"))
  (return 0.0))

(fn `InspectPickUp`
  (bind _returnvalue (`GameplayStatics.GetPlayerController` 0))
  (bind _displaymesh (`self.DisplayMesh`))
  (bind _playercharacter (`self.PlayerCharacter`))
  (bind _displaymesh_2 (`self.DisplayMesh`))
  (bind _playercharacter_2 (`self.PlayerCharacter`))
  (bind _playercharacter_3 (`self.PlayerCharacter`))
  (bind _currentcamera (`/Game/ThirdPerson/Blueprints/BP_ThirdPersonCharacter.CurrentCamera` _playercharacter_2))
  (bind _currentcamera_2 (`/Game/ThirdPerson/Blueprints/BP_ThirdPersonCharacter.CurrentCamera` _playercharacter))
  (bind _itemfp (`/Game/ThirdPerson/Blueprints/BP_ThirdPersonCharacter.ItemFP` _playercharacter_3))
  (`self.DisableInput` (`self.PlayerCharacter`) _returnvalue)
  (`self.EnableInput` _returnvalue)
  (if (== (`/Game/ThirdPerson/Blueprints/BP_ThirdPersonCharacter.CurrentCamera` _playercharacter_3) _itemfp)
    (`self.K2_AttachToComponent` _itemfp "None" "SnapToTarget" "SnapToTarget" "KeepRelative")
    (`PrimitiveComponent.SetSimulatePhysics` _displaymesh false)
    (`PrimitiveComponent.SetCollisionEnabled` _displaymesh "NoCollision")
    (set `/Game/ThirdPerson/Blueprints/BP_ThirdPersonCharacter.CurrentItem` self _playercharacter)
    (`self.K2_SetActorLocation` (+ (`SceneComponent.K2_GetComponentLocation` _currentcamera_2) (* (`KismetMathLibrary.GetForwardVector` (`SceneComponent.K2_GetComponentRotation` _currentcamera_2)) (`self.InsepctDistanceFP`))))
    (else
      (`self.K2_AttachToComponent` (`/Game/ThirdPerson/Blueprints/BP_ThirdPersonCharacter.ItemTP` _playercharacter_3) "None" "SnapToTarget" "SnapToTarget" "KeepRelative")
      (`PrimitiveComponent.SetSimulatePhysics` _displaymesh_2 false)
      (`PrimitiveComponent.SetCollisionEnabled` _displaymesh_2 "NoCollision")
      (set `/Game/ThirdPerson/Blueprints/BP_ThirdPersonCharacter.CurrentItem` self _playercharacter_2)
      (`self.K2_SetActorLocation` (+ (`SceneComponent.K2_GetComponentLocation` _currentcamera) (* (`KismetMathLibrary.GetForwardVector` (`SceneComponent.K2_GetComponentRotation` _currentcamera)) (`self.InsepctDistanceTP`))))))
  (bind _returnvalue_2 (`|CreateWidget` "/Game/06UI/Inventory/Widgets/Inspect/WBP_InspectPickUP.WBP_InspectPickUP_C"))
  (set `self.InspectPickUpText` _returnvalue_2)
  (`/Game/06UI/Inventory/Widgets/Inspect/WBP_InspectPickUP.Add Item name` _returnvalue_2 (`KismetTextLibrary.Conv_NameToText` (`self.ItemName`)))
  (`UserWidget.AddToViewport` _returnvalue_2 0))

(fn `Interact`
  (params (Inventory :type "/Game/06UI/Inventory/AC_InventoryComponent Object Reference") (IDNumber :type Integer) (Character :type "/Game/ThirdPerson/Blueprints/BP_ThirdPersonCharacter Object Reference"))
  (returns (bSucced :type Boolean))
  (bind _returnvalue (`GameplayStatics.GetPlayerController` 0))
  (if (`self.?PickedUP`)
    (set `self.?PickedUP` false)
    (bind _output_get (set `self.PlayerCharacter` Character))
    (bind _currentitem (`/Game/ThirdPerson/Blueprints/BP_ThirdPersonCharacter.CurrentItem` _output_get)
      (:`then`
        (`self.DisableInput` _returnvalue)
        (`self.InspectPickUp` _currentitem))
      (:`else`
        (`self.DisableInput` _returnvalue)
        (bind _output_get_2 (set `/Game/ThirdPerson/Blueprints/BP_ThirdPersonCharacter.CurrentItem` self _output_get))
        (`self.InspectPickUp` _currentitem)
        (`self.InspectPickUp` _output_get_2)))
    (`self.EnableInput` (`self.PlayerCharacter`) _returnvalue)
    (bind _quantity (`/Game/06UI/Inventory/AC_InventoryComponent.ProcessItem` Inventory (make `/Game/06UI/Inventory/F_InventoryItem` (`self.Item`) (`self.Quantity`) null)))
    (if (<= _quantity 0)
      (`self.Destroy item`)
      (return true)
      (else
        (set `self.Quantity` _quantity)
        (return false)))))

(fn `SetLookAt`
  (params (bLookingAt :type Boolean))
  (returns (InteractText :type Text) (Name :type Name))
  (bind (_interacttext _displayname) (defaults `Object` (`self.Item`)))
  (`PrimitiveComponent.SetRenderCustomDepth` (`self.DisplayMesh`) bLookingAt)
  (`SceneComponent.SetVisibility` (`self.Widget`) bLookingAt false)
  (return _interacttext _displayname))

(fn `UserConstructionScript`
  (bind (_displayname _billboardtexture) (defaults `Object` (`self.Item`)))
  (`BillboardComponent.SetSprite` (`self.Billboard`) _billboardtexture)
  (set `self.ItemName` _displayname))