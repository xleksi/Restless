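; Modular climbable ladder that builds itself to a configurable height and tells the player character when to enter or exit at either end.
; The construction script scales the poles, adds instanced rungs and optional screws, and places the top exit area.
; Trigger boxes send messages to the player and toggle top and bottom prompt widgets.
; Four collision events switch active boxes per climb state, with Nope gating the bottom exit.
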(event `self.ReceiveBeginPlay`
  (`/Engine/EditorBlueprintResources/StandardMacros.DoOnce` false
    (:`Completed`
      (`PrimitiveComponent.SetCollisionEnabled` (`self.BottomBox`) "NoCollision")
      (set `self.Nope` false))))

(event `self.EnterBox.OnComponentBeginOverlap`
  (params (OverlappedComponent :type "PrimitiveComponent Object Reference") (OtherActor :type "Actor Object Reference") (OtherComp :type "PrimitiveComponent Object Reference") (OtherBodyIndex :type Integer) (bFromSweep :type Boolean) (SweepResult :type "HitResult Structure (by ref)"))
  ;[1 1 1] Climbing Up
  (if (== OtherActor (`GameplayStatics.GetPlayerCharacter` 0))
    (message `/Game/06UI/AssetsUI/Ladder/BI_Ladder.SetladderInteraction` OtherActor self true)
    (message `/Game/06UI/AssetsUI/Ladder/BI_Ladder.IsNearLadder?` OtherActor true)
    (`SceneComponent.SetVisibility` (`self.WidgetBottom`) true false)))

(event `self.EnterBox.OnComponentEndOverlap`
  (params (OverlappedComponent :type "PrimitiveComponent Object Reference") (OtherActor :type "Actor Object Reference") (OtherComp :type "PrimitiveComponent Object Reference") (OtherBodyIndex :type Integer))
  (if (== OtherActor (`GameplayStatics.GetPlayerCharacter` 0))
    (message `/Game/06UI/AssetsUI/Ladder/BI_Ladder.IsNearLadder?` OtherActor false)
    (`SceneComponent.SetVisibility` (`self.WidgetBottom`) false false)))

(event `self.ExitBox.OnComponentBeginOverlap`
  (params (OverlappedComponent :type "PrimitiveComponent Object Reference") (OtherActor :type "Actor Object Reference") (OtherComp :type "PrimitiveComponent Object Reference") (OtherBodyIndex :type Integer) (bFromSweep :type Boolean) (SweepResult :type "HitResult Structure (by ref)"))
  ;[1 1 1] On Exit Box enterd
  (if (== OtherActor (`GameplayStatics.GetPlayerCharacter` 0))
    (message `/Game/06UI/AssetsUI/Ladder/BI_Ladder.ExitLadderTop` OtherActor (`SceneComponent.K2_GetComponentLocation` (`self.ExitPoint2`)))
    (message `/Game/06UI/AssetsUI/Ladder/BI_Ladder.IsNearLadder?` OtherActor false)))

(event `self.ReturnBox.OnComponentEndOverlap`
  (params (OverlappedComponent :type "PrimitiveComponent Object Reference") (OtherActor :type "Actor Object Reference") (OtherComp :type "PrimitiveComponent Object Reference") (OtherBodyIndex :type Integer))
  (if (== OtherActor (`GameplayStatics.GetPlayerCharacter` 0))
    (message `/Game/06UI/AssetsUI/Ladder/BI_Ladder.IsNearLadder?` OtherActor false)
    (`SceneComponent.SetVisibility` (`self.WidgetTop`) false false)))

(event `self.ReturnBox.OnComponentBeginOverlap`
  (params (OverlappedComponent :type "PrimitiveComponent Object Reference") (OtherActor :type "Actor Object Reference") (OtherComp :type "PrimitiveComponent Object Reference") (OtherBodyIndex :type Integer) (bFromSweep :type Boolean) (SweepResult :type "HitResult Structure (by ref)"))
  ;[1 1 1] Climbing Down
  (if (== OtherActor (`GameplayStatics.GetPlayerCharacter` 0))
    (message `/Game/06UI/AssetsUI/Ladder/BI_Ladder.SetladderInteraction` OtherActor self false)
    (message `/Game/06UI/AssetsUI/Ladder/BI_Ladder.IsNearLadder?` OtherActor true)
    (`SceneComponent.SetVisibility` (`self.WidgetTop`) true false)))

(event `self.BottomBox.OnComponentBeginOverlap`
  (params (OverlappedComponent :type "PrimitiveComponent Object Reference") (OtherActor :type "Actor Object Reference") (OtherComp :type "PrimitiveComponent Object Reference") (OtherBodyIndex :type Integer) (bFromSweep :type Boolean) (SweepResult :type "HitResult Structure (by ref)"))
  ;[1 1 1] Comment
  (if (== OtherActor (`GameplayStatics.GetPlayerCharacter` 0))
    (if (`self.Nope`)
      (message `/Game/06UI/AssetsUI/Ladder/BI_Ladder.ExitLadderBottom` OtherActor (- (`SceneComponent.K2_GetComponentLocation` (`self.LadderBeginningPoint`)) (0.0 0.0 30.0)))
      (message `/Game/06UI/AssetsUI/Ladder/BI_Ladder.IsNearLadder?` OtherActor false))))

(event `/Game/06UI/AssetsUI/Ladder/BI_Ladder.CollisionFromBottom`
  (`PrimitiveComponent.SetCollisionEnabled` (`self.ReturnBox`) "NoCollision")
  (`PrimitiveComponent.SetCollisionEnabled` (`self.ExitBox`) "QueryAndPhysics")
  (`PrimitiveComponent.SetCollisionEnabled` (`self.EnterBox`) "NoCollision")
  (`PrimitiveComponent.SetCollisionEnabled` (`self.BottomBox`) "QueryAndPhysics")
  (set `self.Nope` true))

(event `/Game/06UI/AssetsUI/Ladder/BI_Ladder.CollisionFromTop`
  (`PrimitiveComponent.SetCollisionEnabled` (`self.EnterBox`) "NoCollision")
  (`PrimitiveComponent.SetCollisionEnabled` (`self.ExitBox`) "QueryAndPhysics")
  (`PrimitiveComponent.SetCollisionEnabled` (`self.BottomBox`) "QueryAndPhysics")
  (`PrimitiveComponent.SetCollisionEnabled` (`self.ReturnBox`) "NoCollision")
  (set `self.Nope` true))

(event `/Game/06UI/AssetsUI/Ladder/BI_Ladder.CollisionExitBottom`
  (`PrimitiveComponent.SetCollisionEnabled` (`self.EnterBox`) "QueryAndPhysics")
  (`PrimitiveComponent.SetCollisionEnabled` (`self.ExitBox`) "QueryAndPhysics")
  (`PrimitiveComponent.SetCollisionEnabled` (`self.BottomBox`) "NoCollision")
  (`PrimitiveComponent.SetCollisionEnabled` (`self.ReturnBox`) "QueryAndPhysics")
  (set `self.Nope` false))

(event `/Game/06UI/AssetsUI/Ladder/BI_Ladder.CollisionExitTop`
  (`PrimitiveComponent.SetCollisionEnabled` (`self.ReturnBox`) "QueryAndPhysics")
  (`PrimitiveComponent.SetCollisionEnabled` (`self.EnterBox`) "QueryAndPhysics")
  (`PrimitiveComponent.SetCollisionEnabled` (`self.BottomBox`) "NoCollision")
  (`PrimitiveComponent.SetCollisionEnabled` (`self.ExitBox`) "NoCollision")
  (set `self.Nope` false))

(fn `SetLadderExitArea`
  (bind _returnvalue (* (`self.LadderHeight`) 100.0))
  (`SceneComponent.K2_SetRelativeLocation` (`self.ExitBox`) (`KismetMathLibrary.MakeVector` -30.0 0.0 (+ _returnvalue (`self.ExitBoxOffset`))) false false)
  (`SceneComponent.K2_SetRelativeLocation` (`self.LadderExitArea`) (`KismetMathLibrary.MakeVector` 0.0 0.0 _returnvalue) false false))

(fn `UserConstructionScript`
  (`SceneComponent.SetRelativeScale3D` (`self.RightLadderPole`) (`KismetMathLibrary.MakeVector` 0.1 0.1 (`self.LadderHeight`)))
  (`SceneComponent.SetRelativeScale3D` (`self.LeftLadderPole`) (`KismetMathLibrary.MakeVector` 0.1 0.1 (`self.LadderHeight`)))
  (while (< (`self.CompareHeight`) (* (`self.LadderHeight`) 100.0))
    (`self.AddBarsAndScrews`))
  (`self.SetLadderExitArea`))