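; BP_InstructionPlaceholder is a UI placeholder actor that displays instruction text in the world through text render components.
; On BeginPlay it copies four text variables into four TextRender components, one per component.
; The construction script is empty, so the text is applied only at runtime.
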(event `self.ReceiveBeginPlay`
  (`TextRenderComponent.K2_SetText` (`self.TextRender`) (`self.Text1`))
  (`TextRenderComponent.K2_SetText` (`self.TextRender1`) (`self.Text1_0`))
  (`TextRenderComponent.K2_SetText` (`self.TextRender2`) (`self.Text1_1`))
  (`TextRenderComponent.K2_SetText` (`self.TextRender3`) (`self.Text1_2`)))

(fn `UserConstructionScript`)